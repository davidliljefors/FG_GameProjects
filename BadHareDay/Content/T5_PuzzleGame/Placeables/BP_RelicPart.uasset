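; BP_RelicPart is a placeable relic piece for the puzzle game, collected in a fixed sequence by order number.
; On pickup it plays a poof and sound, hides the mesh, disables collision, notifies every relic part, then destroys itself after a short delay.
; The part with the next order number reveals its mesh and sparkles and enables query collision.
; The construction script reveals the part flagged as first.
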(event `self.OnPickedUp`
  (params (PickedBy :type "GravityCharacter Object Reference"))
  ;[1 1 1] On picked up
  (`ActorComponent.Activate` (`self.poof`) false)
  (`GameplayStatics.PlaySound2D` "/Game/T5_PuzzleGame/Audio/CUE_Pickup.CUE_Pickup" 1.0 1.0 0.0 null null)
  (`PrimitiveComponent.SetCollisionEnabled` (`self.SphereCollision`) "NoCollision")
  (`PrimitiveComponent.SetCollisionEnabled` (`self.Mesh`) "NoCollision")
  (`SceneComponent.SetVisibility` (`self.Mesh`) false false)
  (bind _outactors (`GameplayStatics.GetAllActorsOfClass` "BP_RelicPart_C"))
  (for _array_element _outactors
    (`/Engine/EditorBlueprintResources/StandardMacros.IsValid` _array_element
      (:`Is Valid`
        (`self.CheckRender` _array_element (`self.OrderNumber`)))))
  (`KismetSystemLibrary.Delay` 0.5)
  (`self.K2_DestroyActor`))

(event `CheckRender`
  (params (lastRelic :type Integer))
  ;[1 1 1] Set visibility
  (bind _result (`/Engine/EditorBlueprintResources/StandardMacros.IncrementInt` lastRelic)
    (:`  `
      (if (== _result (`self.OrderNumber`))
        (`SceneComponent.SetVisibility` (`self.Mesh`) true false)
        (`SceneComponent.SetVisibility` (`self.Sparkles`) true false)
        (`PrimitiveComponent.SetCollisionEnabled` (`self.SphereCollision`) "QueryOnly")
        (`ActorComponent.Activate` (`self.Sparkles`) true)))))

(fn `UserConstructionScript`
  (if (`self.IsFirst`)
    (`SceneComponent.SetVisibility` (`self.Mesh`) true false)
    (`SceneComponent.SetVisibility` (`self.Sparkles`) true false)
    (`PrimitiveComponent.SetCollisionEnabled` (`self.SphereCollision`) "QueryOnly")))