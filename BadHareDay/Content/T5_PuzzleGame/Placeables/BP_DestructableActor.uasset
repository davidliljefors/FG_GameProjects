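; Breakable puzzle placeable that shatters when a fast-moving big-rock gravity-swappable push box enters its trigger box.
; The impact notifies the rock, plays sound and camera shake, damages the destructible mesh, optionally destroys the rock, drops blocking collision, then hides the debris after a delay.
; Player checkpoint events save transform, visibility and collision; respawn restores them and resets the destructible mesh if it was visible.
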(event `self.ReceiveBeginPlay`
  (`DestructibleComponent.SetDestructibleMesh` (`self.Destructible`) (`self.DestructableMesh`))
  (`SceneComponent.SetVisibility` (`self.StaticMesh`) false false)
  (bind _asbp_player (cast `/Game/T5_PuzzleGame/Characters/BP_Player` (`GameplayStatics.GetPlayerCharacter` 0)))
  (bind _output_get (set `self.PlayerRef` _asbp_player))
  (add `/Game/T5_PuzzleGame/Characters/BP_Player.OnCheckPointEnter` _output_get (delegate `OnCheckPointEnter`))
  (add `/Game/T5_PuzzleGame/Characters/BP_Player.OnPlayerRespawn` _output_get (delegate `OnPlayerRespawn`)))

(event `OnCheckPointEnter`
  ;[1 1 1] OnCheckPointEnter
  (set `self.SavedTransform` (`self.GetTransform`))
  (set `self.SavedVisible` (`SceneComponent.bVisible` (`self.DefaultSceneRoot`)))
  (set `self.SavedCollision` (`PrimitiveComponent.GetCollisionEnabled` (`self.StaticMesh`))))

(event `OnPlayerRespawn`
  ;[1 1 1] OnPlayerRespawn
  (`self.K2_SetActorTransform` (`self.SavedTransform`) false true)
  (`SceneComponent.SetVisibility` (`self.DefaultSceneRoot`) (`self.SavedVisible`) true)
  (`PrimitiveComponent.SetCollisionEnabled` (`self.StaticMesh`) (`self.SavedCollision`))
  (if (`self.SavedVisible`)
    (`DestructibleComponent.SetDestructibleMesh` (`self.Destructible`) (`self.DestructableMesh`))
    (`SceneComponent.SetVisibility` (`self.StaticMesh`) false false)))

(event `self.Box.OnComponentBeginOverlap`
  (params (OverlappedComponent :type "PrimitiveComponent Object Reference") (OtherActor :type "Actor Object Reference") (OtherComp :type "PrimitiveComponent Object Reference") (OtherBodyIndex :type Integer) (bFromSweep :type Boolean) (SweepResult :type "HitResult Structure (by ref)"))
  (bind _returnvalue (`self.K2_GetActorLocation` OtherActor))
  (bind _destructible (`self.Destructible`))
  (if (== (`GameplayStatics.GetObjectClass` OtherActor) "/Game/T5_PuzzleGame/Placeables/Interactables/BP_GravitySwappablePushBox_Big_Rock.BP_GravitySwappablePushBox_Big_Rock_C")
    (if (> (`KismetMathLibrary.VSize` (`self.GetVelocity` OtherActor)) 1000.0)
      (bind _asbp_gravity_swappable_push_box_base (cast `/Game/T5_PuzzleGame/Core/BP_GravitySwappablePushBoxBase` OtherActor))
      (`GameplayStatics.PlaySound2D` "/Game/T5_PuzzleGame/Audio/CUE_LayerBreak.CUE_LayerBreak" 1.0 1.0 0.0 null null)
      (`/Game/T5_PuzzleGame/Core/BP_GravitySwappablePushBoxBase.OnBreakLayer` _asbp_gravity_swappable_push_box_base)
      (`/Game/T5_PuzzleGame/Core/BPFL_ControllerFunctions.Play Camera Shake`)
      (`KismetSystemLibrary.Delay` 0.1)
      (`DestructibleComponent.ApplyDamage` (`self.Destructible`) 5555.0 _returnvalue (- _returnvalue (`KismetMathLibrary.Vector_Zero`)) 5555.0)
      (if (`self.bShouldDestroyBox`)
        (`self.SetLifeSpan` OtherActor 0.5))
      (`PrimitiveComponent.SetCollisionEnabled` (`self.StaticMesh`) "NoCollision")
      (`PrimitiveComponent.SetCollisionResponseToChannel` _destructible "ECC_Pawn" "ECR_Ignore")
      (`PrimitiveComponent.SetCollisionResponseToChannel` _destructible "ECC_GameTraceChannel5" "ECR_Ignore")
      (`KismetSystemLibrary.Delay` 3.0)
      (`SceneComponent.SetVisibility` (`self.DefaultSceneRoot`) false true))))

(fn `UserConstructionScript`)