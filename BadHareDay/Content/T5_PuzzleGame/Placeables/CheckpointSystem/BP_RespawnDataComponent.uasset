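; BP_RespawnDataComponent stores checkpoint respawn data for its owning actor in the puzzle game.
; It records the owner's transform and GravitySwapComponent flip state at BeginPlay, then re-saves only the flip state on checkpoint entry.
; OnRest is empty.
; Disconnected restore logic would respawn big push boxes and swap them in BP_RespawnManger's list, or teleport other owners' meshes back with saved gravity.
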(event `CheckPointInterface.OnRest`)

(event `self.ReceiveBeginPlay`
  (set `self.StartActorLocation` (`Actor.GetTransform` (`self.GetOwner`)))
  (set `self.FlipGravitySave` (`GravitySwapComponent.bFlipGravity` (`Actor.GetComponentByClass` (`self.GetOwner`) "/Script/GP2_Team5.GravitySwapComponent"))))

(event `CheckPointInterface.OnEnterCheckPoint`
  (params (ActorCaller :type "Actor Object Reference") (CheckpointCaller :type "Actor Object Reference"))
  (bind _returnvalue (`Actor.GetComponentByClass` (`self.GetOwner`) "/Script/GP2_Team5.GravitySwapComponent"))
  (`/Engine/EditorBlueprintResources/StandardMacros.IsValid` _returnvalue
    (:`Is Valid`
      (set `self.FlipGravitySave` (`GravitySwapComponent.bFlipGravity` _returnvalue)))
    (:`Is Not Valid`
      (`KismetSystemLibrary.PrintString` "bnm,ghjklghjkghjkghjkhjkg"))))