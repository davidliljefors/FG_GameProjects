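; BP_Checkpoint is a placeable checkpoint trigger for the puzzle game's checkpoint system.
; When a living BP_Player overlaps its Box, it waits briefly, then calls the player's CallOnCheckPointEnter and prints a debug message.
; It caches BP_RespawnManger on BeginPlay, but the direct OnEnterCheckPoint call to that manager is disconnected and never runs.
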(event `self.ReceiveBeginPlay`
  (bind _returnvalue (`GameplayStatics.GetActorOfClass` "/Game/T5_PuzzleGame/Placeables/CheckpointSystem/BP_RespawnManger.BP_RespawnManger_C"))
  (set `self.BP_RespawnManger` _returnvalue))

(event `self.Box.OnComponentBeginOverlap`
  (params (OverlappedComponent :type "PrimitiveComponent Object Reference") (OtherActor :type "Actor Object Reference") (OtherComp :type "PrimitiveComponent Object Reference") (OtherBodyIndex :type Integer) (bFromSweep :type Boolean) (SweepResult :type "HitResult Structure (by ref)"))
  (bind _asbp_player (cast `/Game/T5_PuzzleGame/Characters/BP_Player` OtherActor))
  (if (not (`/Game/T5_PuzzleGame/Characters/BP_Player.IsDead` _asbp_player))
    (`KismetSystemLibrary.Delay` 0.3)
    (`/Game/T5_PuzzleGame/Characters/BP_Player.OnCheckPointEnter` _asbp_player)
    (`KismetSystemLibrary.PrintString` "Enter Check Point!")))

(fn `UserConstructionScript`)