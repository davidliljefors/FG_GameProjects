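; Respawn manager actor for the puzzle game's checkpoint system, handling checkpoint saves and level resets.
; On BeginPlay it gathers tagged actors, creates and saves a BP_SaveGameScript, and caches the player.
; Entering a checkpoint saves the player's location and stores each tagged actor's mesh transform in its BP_RespawnDataComponent.
; Reset calls OnRest on those components and re-saves; level finish only prints a debug message.
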(event `self.ReceiveBeginPlay`
  ;[1 1 1] Start
  (`self.GetAllRefrances`
    (:`Out`
      (bind _output_get (set `self.CurrentPlayerLoction` (`self.K2_GetActorLocation` (`self.PlayerCharacterRefrance`))))
      (set `/Game/T5_PuzzleGame/Placeables/CheckpointSystem/BP_SaveGameScript.SavedPlayerLocation` _output_get (`self.BP_SaveGame`)))))

(event `CheckPointInterface.OnEnterCheckPoint`
  (params (ActorCaller :type "Actor Object Reference") (CheckpointCaller :type "Actor Object Reference"))
  (bind _bp_savegame (`self.BP_SaveGame`))
  (bind _playercharacterrefrance (`self.PlayerCharacterRefrance`))
  ;[1 1 1] Setting checkpoints
  (set `self.CallerRefrances` ActorCaller)
  (set `self.CheckpointCaller` CheckpointCaller)
  (set `self.CurrentPlayerLoction` (`self.K2_GetActorLocation` _playercharacterrefrance))
  (message `CheckPointInterface.OnEnterCheckPoint` _playercharacterrefrance null null)
  (set `self.LastCaller` (`self.CallerRefrances`))
  (bind _output_get (set `self.CheckpointSaved` (`self.CheckpointCaller`)))
  (`KismetSystemLibrary.PrintString` (`KismetSystemLibrary.GetDisplayName` _output_get))
  (`GameplayStatics.LoadGameFromSlot` (`self.SaveGameSlot`))
  (set `/Game/T5_PuzzleGame/Placeables/CheckpointSystem/BP_SaveGameScript.SavedPlayerLocation` (`self.CurrentPlayerLoction`) _bp_savegame)
  (`GameplayStatics.SaveGameToSlot` _bp_savegame (`self.SaveGameSlot`))
  (for _array_element (`self.AllActors`)
    (`/Engine/EditorBlueprintResources/StandardMacros.IsValid` _array_element
      (:`Is Valid`
        (bind _returnvalue (`self.GetComponentByClass` _array_element "/Game/T5_PuzzleGame/Placeables/CheckpointSystem/BP_RespawnDataComponent.BP_RespawnDataComponent_C"))
        (`/Engine/EditorBlueprintResources/StandardMacros.IsValid` _returnvalue
          (:`Is Valid`
            (message `CheckPointInterface.OnEnterCheckPoint` _returnvalue null null)
            (set `/Game/T5_PuzzleGame/Placeables/CheckpointSystem/BP_RespawnDataComponent.StartActorLocation` (`SceneComponent.K2_GetComponentToWorld` (`self.GetComponentByClass` _array_element "/Script/Engine.StaticMeshComponent")) _returnvalue)))))))

(event `CheckPointInterface.OnRest`
  ;[1 1 1] Rest game
  (`KismetSystemLibrary.PrintString` "On Reset called for whole level!")
  (`GameplayStatics.LoadGameFromSlot` (`self.SaveGameSlot`))
  (for _array_element (`self.AllActors`)
    (`/Engine/EditorBlueprintResources/StandardMacros.IsValid` _array_element
      (:`Is Valid`
        (bind _returnvalue (`self.GetComponentByClass` _array_element "/Game/T5_PuzzleGame/Placeables/CheckpointSystem/BP_RespawnDataComponent.BP_RespawnDataComponent_C"))
        (`/Engine/EditorBlueprintResources/StandardMacros.IsValid` _returnvalue
          (:`Is Valid`
            (`KismetSystemLibrary.PrintString` (`KismetSystemLibrary.GetDisplayName` _returnvalue))
            (`CheckPointInterface.OnRest` _returnvalue)
            (`GameplayStatics.SaveGameToSlot` (`self.BP_SaveGame`) (`self.SaveGameSlot`))
            (`KismetSystemLibrary.PrintString` "Save state cleared!"))))
      (:`Is Not Valid`
        (`KismetSystemLibrary.PrintString` "Actor in rest loop not valid")))))

(event `CheckPointInterface.OnFinnishlevel`
  ;[1 1 1] Finnish Level
  (`KismetSystemLibrary.PrintString` "Finnish level called"))

(fn `UserConstructionScript`)