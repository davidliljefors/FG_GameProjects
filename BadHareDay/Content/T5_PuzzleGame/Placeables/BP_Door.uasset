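; BP_Door is a sliding puzzle door that opens when its linked Switch is pressed and closes when it is released.
; On BeginPlay it binds to the switch, stores its location as closed, and sets the open position to the rotated slide offset.
; Paired DoOnce gates alternate playing and reversing a timeline that lerps between both positions.
; Its construction script orients it on a sphere, optionally upside down.
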(event `self.ReceiveBeginPlay`
  (bind _switch (`self.Switch`))
  (add `/Game/T5_PuzzleGame/Placeables/BP_FloorSwitch.OnPressed` _switch (delegate `OnSwitchPressed`))
  (add `/Game/T5_PuzzleGame/Placeables/BP_FloorSwitch.OnUnPressed` _switch (delegate `OnSwitchReleased`))
  (set `self.ClosedPos` (`self.K2_GetActorLocation`))
  (set `self.OpenPos` (`KismetMathLibrary.GreaterGreater_VectorRotator` (`self.DoorSlideOffset`) (`self.K2_GetActorRotation`))))

(event `OnSwitchPressed`
  (`/Engine/EditorBlueprintResources/StandardMacros.DoOnce` false :!label _label
    (:`Completed`
      (`|ExecutionSequence`
        (:`then_0`
          (goto _label_3 :!via `Reset`))
        (:`then_1`
          (bind (_direction _t) (`Timeline|DoorOpening` :!label _label_2)
            (:`Update`
              (`self.K2_SetActorLocation` (`KismetMathLibrary.VLerp` (`self.ClosedPos`) (`self.OpenPos`) _t)))
            (:`Finished`
              (switch `ETimelineDirection` _direction
                (:`Forward`
                  (`KismetSystemLibrary.PrintString` "Door fully opened"))))))))))

(event `OnSwitchReleased`
  (`/Engine/EditorBlueprintResources/StandardMacros.DoOnce` true :!label _label_3
    (:`Completed`
      (`|ExecutionSequence`
        (:`then_0`
          (goto _label :!via `Reset`))
        (:`then_1`
          (goto _label_2 :!via `Reverse`))))))

(fn `UserConstructionScript`
  (`/Game/T5_PuzzleGame/Core/BPFL_RotationFunctions.Set Actor Rotation On Sphere` self (`self.bUpsideDown`)))