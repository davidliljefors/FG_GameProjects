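; BP_TutorialText is a placeable trigger in the puzzle game that shows a tutorial text widget once when overlapped.
; After a delay it creates WPB_TutorialText with the selected tutorial, then timelines drive its opacity on either side of a configurable display time.
; When the second timeline finishes, it removes the widget and destroys itself.
; The end-overlap event is empty, and logic to zero the display time is disconnected.
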(event `self.ReceiveActorBeginOverlap`
  (params (OtherActor :type "Actor Object Reference"))
  (`/Engine/EditorBlueprintResources/StandardMacros.DoOnce` false
    (:`Completed`
      (`KismetSystemLibrary.Delay` (`self.Delay`))
      (bind _returnvalue (`|CreateWidget` "/Game/T5_PuzzleGame/UserInterfaces/WPB_TutorialText.WPB_TutorialText_C"))
      (bind _output_get (set `self.WidgetVar` _returnvalue))
      (set `/Game/T5_PuzzleGame/UserInterfaces/WPB_TutorialText.Select Tutorial` (`self.SelectTut`) _output_get)
      (`UserWidget.AddToViewport` _output_get 0)
      (bind (_direction _newtrack_0) (`Timeline|Timeline_0` :!via `PlayFromStart`)
        (:`Update`
          (`Widget.SetRenderOpacity` (`self.WidgetVar`) _newtrack_0))
        (:`Finished`
          (`KismetSystemLibrary.Delay` (`self.ShowTime`))
          (bind (_direction_2 _newtrack_0_2) (`Timeline|Timeline_1`)
            (:`Update`
              (`Widget.SetRenderOpacity` (`self.WidgetVar`) _newtrack_0_2))
            (:`Finished`
              (`Widget.RemoveFromParent` (`self.WidgetVar`))
              (set `self.WidgetVar` (`self.EmptyWidget`))
              (`self.K2_DestroyActor`))))))))

(event `self.ReceiveActorEndOverlap`
  (params (OtherActor :type "Actor Object Reference")))

(fn `UserConstructionScript`)