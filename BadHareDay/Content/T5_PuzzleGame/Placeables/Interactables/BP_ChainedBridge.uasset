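; BP_ChainedBridge is a clickable bridge placeable for the puzzle game, with four cables attached to a shared Billboard anchor in the construction script.
; ClickInteract toggles a temporary point light and marks the bridge selected, and its reset event clears both.
; The Stabalizer volume zeroes the velocity of overlapping actors' meshes to steady boxes on the bridge.
; SetGrondCollision sets the response of four capsules to a custom trace channel.
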(event `self.ReceiveBeginPlay`
  (`SceneComponent.SetVisibility` (`self.TempPointLight`) (`self.bLightOn`) false))

(event `self.ClickInteract.OnClickInteract`
  (bind _output_get (set `self.bLightOn` (not (`self.bLightOn`))))
  (`SceneComponent.SetVisibility` (`self.TempPointLight`) _output_get false)
  (set `self.bSelected` true))

(event `self.ClickInteract.OnResetClickInteract`
  (bind _output_get (set `self.bLightOn` false))
  (`SceneComponent.SetVisibility` (`self.TempPointLight`) _output_get false)
  (set `self.bSelected` false))

(event `self.Stabalizer.OnComponentBeginOverlap`
  (params (OverlappedComponent :type "PrimitiveComponent Object Reference") (OtherActor :type "Actor Object Reference") (OtherComp :type "PrimitiveComponent Object Reference") (OtherBodyIndex :type Integer) (bFromSweep :type Boolean) (SweepResult :type "HitResult Structure (by ref)"))
  ;[1 1 1] Stabalize boxes on bridges
  (`PrimitiveComponent.SetAllPhysicsLinearVelocity` (`self.GetComponentByClass` OtherActor "/Script/Engine.StaticMeshComponent") (0.0 0.0 0.0) false))

(fn `Set Grond Collision`
  (params (CollisionEnabled :type "ECollisionResponse Enum" :default "ECR_Ignore"))
  (`PrimitiveComponent.SetCollisionResponseToChannel` (`self.Capsule`) "ECC_GameTraceChannel2" CollisionEnabled)
  (`PrimitiveComponent.SetCollisionResponseToChannel` (`self.Capsule1`) "ECC_GameTraceChannel2" CollisionEnabled)
  (`PrimitiveComponent.SetCollisionResponseToChannel` (`self.Capsule3`) "ECC_GameTraceChannel2" CollisionEnabled)
  (`PrimitiveComponent.SetCollisionResponseToChannel` (`self.Capsule2`) "ECC_GameTraceChannel2" CollisionEnabled))

(fn `UserConstructionScript`
  (bind _billboard (`self.Billboard`))
  (`CableComponent.SetAttachEndToComponent` (`self.Cable`) _billboard "None")
  (`CableComponent.SetAttachEndToComponent` (`self.Cable1`) _billboard "None")
  (`CableComponent.SetAttachEndToComponent` (`self.Cable2`) _billboard "None")
  (`CableComponent.SetAttachEndToComponent` (`self.Cable3`) _billboard "None"))