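; Placeable gravity swapper for the puzzle game that flips the player's gravity or switches a gravity-swappable push box on overlap.
; For the player, it releases any grabbed box, toggles flipped gravity, halts movement and briefly disables input.
; Push boxes are released, then lerp-switched toward the swapper's position at X zero.
; Both paths play sound and FX, with a timed cooldown and temporary collision disable preventing immediate retriggering.
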(event `self.ReceiveBeginPlay`
  (bind _asbp_gravity_character_base (cast `/Game/T5_PuzzleGame/Core/BP_GravityCharacterBase` (`GameplayStatics.GetPlayerCharacter` 0)))
  (set `self.PlayerRef` _asbp_gravity_character_base))

(event `self.Box.OnComponentBeginOverlap`
  (params (OverlappedComponent :type "PrimitiveComponent Object Reference") (OtherActor :type "Actor Object Reference") (OtherComp :type "PrimitiveComponent Object Reference") (OtherBodyIndex :type Integer) (bFromSweep :type Boolean) (SweepResult :type "HitResult Structure (by ref)"))
  (bind _returnvalue (`GameplayStatics.GetPlayerController` 0))
  (bind _playerref (`self.PlayerRef`))
  (bind _playerref_2 (`self.PlayerRef`))
  (bind _currentgrabbingbox (`GravityCharacter.CurrentGrabbingBox` _playerref))
  (bind _gravityswap (`/Game/T5_PuzzleGame/Core/BP_GravityCharacterBase.GravitySwap` _playerref_2))
  (if (`self.SwapCooldown`)
    _
    (elif (== OtherActor (`self.PlayerRef`))
      (`|ExecutionSequence`
        (:`then_0`
          (`GameplayStatics.PlaySound2D` "/Game/T5_PuzzleGame/Audio/GravitySwap_Cue.GravitySwap_Cue" 1.0 1.0 0.0 null null)
          (`ActorComponent.Activate` (`self.ActivateFX`) false)
          (`GravityCharacter.ResetWalkSpeed` _playerref)
          ;[1 1 1] Player
          (`/Engine/EditorBlueprintResources/StandardMacros.IsValid` _currentgrabbingbox
            (:`Is Valid`
              (`/Game/T5_PuzzleGame/Core/BP_ApproachGrabComponent.Release` (`self.GetComponentByClass` (`ActorComponent.GetOwner` _currentgrabbingbox) "/Game/T5_PuzzleGame/Core/BP_ApproachGrabComponent.BP_ApproachGrabComponent_C")))
            (:`Is Not Valid`
              _))
          (`GravitySwappable.SetFlipGravity` _gravityswap (not (`GravitySwappable.GetFlipGravity` _gravityswap)))
          (`MovementComponent.StopMovementImmediately` (`Pawn.GetMovementComponent` _playerref_2))
          (`self.DisableInput` _playerref_2 _returnvalue)
          (`KismetSystemLibrary.Delay` (`self.InputDisableDuration`))
          (`self.EnableInput` _playerref_2 _returnvalue)
          ;[1 1 1] Collision disable for duration after being activated.
          (`PrimitiveComponent.SetCollisionEnabled` (`self.Box`) "NoCollision" :!label _label)
          (`KismetSystemLibrary.Delay` 1.0)
          (`PrimitiveComponent.SetCollisionEnabled` (`self.Box`) "QueryAndPhysics"))
        (:`then_1`
          (set `self.SwapCooldown` true)
          (`KismetSystemLibrary.Delay` 1.0)
          (set `self.SwapCooldown` false)))
      (else
        (bind _asbp_gravity_swappable_push_box_base (cast `/Game/T5_PuzzleGame/Core/BP_GravitySwappablePushBoxBase` OtherActor))
        (`|ExecutionSequence`
          (:`then_0`
            (`GravityCharacter.ResetWalkSpeed` (`self.PlayerRef`))
            ;[1 1 1] PushBox
            (`GameplayStatics.PlaySound2D` "/Game/T5_PuzzleGame/Audio/GravitySwap_Cue.GravitySwap_Cue" 1.0 1.0 0.0 null null)
            (`ActorComponent.Activate` (`self.ActivateFX`) false)
            (`/Game/T5_PuzzleGame/Core/BP_ApproachGrabComponent.Release` (`/Game/T5_PuzzleGame/Core/BP_GravitySwappablePushBoxBase.BP_ApproachGrabComponent` _asbp_gravity_swappable_push_box_base))
            (`/Game/T5_PuzzleGame/Core/BP_GravitySwappablePushBoxBase.LerpGravitySwitch` _asbp_gravity_swappable_push_box_base (`KismetMathLibrary.MakeVector` 0.0 (.y (`self.K2_GetActorLocation`)) (.z (`self.K2_GetActorLocation`))) self)
            (goto _label))
          (:`then_1`
            (set `self.SwapCooldown` true)
            (`KismetSystemLibrary.Delay` 1.0)
            (set `self.SwapCooldown` false)))))))

(fn `UserConstructionScript`)