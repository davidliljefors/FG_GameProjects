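; Large grabbable, gravity-swappable push box for the puzzle game, extending a parent Blueprint with feedback effects.
; Interactable sparkles switch off while grabbed and return on release.
; Click highlight states toggle a child-actor arrow, placed and oriented along the radial axis through world origin according to FlipGravity.
; Four capsules share a speed-gated, cooldown-limited impact sound, choosing rock or wood by checking for the Rock subclass.
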(event `DEACTIVATEsPARKLS`
  (`ActorComponent.Deactivate` (`self.InteractableSparkles`)))

(event `activateSparks`
  (`ActorComponent.Activate` (`self.InteractableSparkles`) false))

(event `self.ReceiveBeginPlay`
  (bind _bp_approachgrabcomponent (`self.BP_ApproachGrabComponent`))
  (add `/Game/T5_PuzzleGame/Core/BP_ApproachGrabComponent. OnGrabbed` _bp_approachgrabcomponent (delegate `DEACTIVATEsPARKLS`))
  (add `/Game/T5_PuzzleGame/Core/BP_ApproachGrabComponent.OnReleased` _bp_approachgrabcomponent (delegate `activateSparks`))
  (`parent.ReceiveBeginPlay`)
  (bind _asbp_arrow (cast `/Game/T5_PuzzleGame/Placeables/Interactables/BP_Arrow` (`ChildActorComponent.ChildActor` (`self.ArrowComp`))))
  (set `self.ArrowVar` _asbp_arrow)
  (add `ClickInteractComponent.OnActivateHighlight` (`self.ClickInteract`) (delegate `ArrowEv`)))

(event `ArrowEv`
  (params (HightlightType :type "EOutlineType Enum" :default "None"))
  (bind _arrowvar (`self.ArrowVar`))
  (switch `EOutlineType` HightlightType
    (:`None`
      (`/Game/T5_PuzzleGame/Placeables/Interactables/BP_Arrow.Deactivate` _arrowvar :!label _label))
    (:`Hover`
      (`/Game/T5_PuzzleGame/Placeables/Interactables/BP_Arrow.Activate` _arrowvar (select `bool` (`GravitySwapComponent.bFlipGravity` (`self.GravitySwap`)) :`false` (+ (`SceneComponent.K2_GetComponentLocation` (`self.StaticMesh`)) (* (`KismetMathLibrary.GetDirectionUnitVector` (0.0 0.0 0.0) (`SceneComponent.K2_GetComponentLocation` (`self.StaticMesh`))) 190.0)) :`true` (+ (`SceneComponent.K2_GetComponentLocation` (`self.StaticMesh`)) (* (`KismetMathLibrary.GetDirectionUnitVector` (`SceneComponent.K2_GetComponentLocation` (`self.StaticMesh`))) 10.0))) (select `bool` (`GravitySwapComponent.bFlipGravity` (`self.GravitySwap`)) :`false` (`KismetMathLibrary.MakeRotFromZ` (`KismetMathLibrary.GetDirectionUnitVector` (0.0 0.0 0.0) (`SceneComponent.K2_GetComponentLocation` (`self.StaticMesh`)))) :`true` (`KismetMathLibrary.MakeRotFromZ` (`KismetMathLibrary.GetDirectionUnitVector` (`SceneComponent.K2_GetComponentLocation` (`self.StaticMesh`))))) :!label _label_2))
    (:`Selected`
      (goto _label_2))
    (:`Swappable`
      (goto _label_2))
    (:`NonSwappable`
      (goto _label))))

(event `self.StaticMesh.OnComponentHit`
  (params (HitComponent :type "PrimitiveComponent Object Reference") (OtherActor :type "Actor Object Reference") (OtherComp :type "PrimitiveComponent Object Reference") (NormalImpulse :type "Vector Structure") (Hit :type "HitResult Structure (by ref)")))

(event `self.Capsule.OnComponentHit`
  (params (HitComponent :type "PrimitiveComponent Object Reference") (OtherActor :type "Actor Object Reference") (OtherComp :type "PrimitiveComponent Object Reference") (NormalImpulse :type "Vector Structure") (Hit :type "HitResult Structure (by ref)"))
  (if (and (> (`KismetMathLibrary.VSize` (`SceneComponent.GetComponentVelocity` (`self.StaticMesh`))) 50.0) (`self.SoundCooldown`)) :!label _label_3
    (set `self.SoundCooldown` false)
    (if (== (`GameplayStatics.GetObjectClass` self) "/Game/T5_PuzzleGame/Placeables/Interactables/BP_GravitySwappablePushBox_Big_Rock.BP_GravitySwappablePushBox_Big_Rock_C")
      (`GameplayStatics.PlaySound2D` "/Game/T5_PuzzleGame/Audio/CUE_RockImpact.CUE_RockImpact" 1.0 1.0 0.0 null null)
      (else
        (`GameplayStatics.PlaySound2D` "/Game/T5_PuzzleGame/Audio/CUE_WoodImpact.CUE_WoodImpact" 1.0 1.0 0.0 null null)))
    (`KismetSystemLibrary.Delay` 0.2)
    (set `self.SoundCooldown` true)))

(event `self.Capsule1.OnComponentHit`
  (params (HitComponent :type "PrimitiveComponent Object Reference") (OtherActor :type "Actor Object Reference") (OtherComp :type "PrimitiveComponent Object Reference") (NormalImpulse :type "Vector Structure") (Hit :type "HitResult Structure (by ref)"))
  (goto _label_3))

(event `self.Capsule2.OnComponentHit`
  (params (HitComponent :type "PrimitiveComponent Object Reference") (OtherActor :type "Actor Object Reference") (OtherComp :type "PrimitiveComponent Object Reference") (NormalImpulse :type "Vector Structure") (Hit :type "HitResult Structure (by ref)"))
  (goto _label_3))

(event `self.Capsule3.OnComponentHit`
  (params (HitComponent :type "PrimitiveComponent Object Reference") (OtherActor :type "Actor Object Reference") (OtherComp :type "PrimitiveComponent Object Reference") (NormalImpulse :type "Vector Structure") (Hit :type "HitResult Structure (by ref)"))
  (goto _label_3))

(fn `UserConstructionScript`
  (`parent.UserConstructionScript`))