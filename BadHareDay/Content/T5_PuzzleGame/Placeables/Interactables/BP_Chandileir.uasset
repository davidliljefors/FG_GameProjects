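; BP_Chandileir is a chandelier interactable for the puzzle game that stops push boxes that hit it.
; When its ClickBox is hit by an actor whose class is exactly BP_GravitySwappablePushBoxBase, it zeroes that box's static mesh linear velocity.
; It overrides IsFallingOntoPlayer to always return false, so it never reports itself as falling onto the player.
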(event `self.ClickBox.OnComponentHit`
  (params (HitComponent :type "PrimitiveComponent Object Reference") (OtherActor :type "Actor Object Reference") (OtherComp :type "PrimitiveComponent Object Reference") (NormalImpulse :type "Vector Structure") (Hit :type "HitResult Structure (by ref)"))
  (if (== (`GameplayStatics.GetObjectClass` OtherActor) "/Game/T5_PuzzleGame/Core/BP_GravitySwappablePushBoxBase.BP_GravitySwappablePushBoxBase_C")
    (`PrimitiveComponent.SetAllPhysicsLinearVelocity` (`self.GetComponentByClass` OtherActor "/Script/Engine.StaticMeshComponent") (0.0 0.0 0.0) false)))

(fn `IsFallingOntoPlayer`
  (params (Player :type "GravityCharacter Object Reference"))
  (returns (Value :type Boolean))
  (return false))

(fn `UserConstructionScript`
  (`parent.UserConstructionScript`))