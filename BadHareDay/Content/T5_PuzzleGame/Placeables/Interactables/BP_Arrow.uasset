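; BP_Arrow is a puzzle-game arrow indicator that stays hidden until activated at a given location and rotation.
; Activate shows the mesh with an outline material and custom depth stencil, then a Timeline lerps it between the start point and an offset along its up vector.
; Deactivate hides the mesh and stops the Timeline.
; A delayed activate/deactivate test loop remains in the graph but is unconnected.
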(event `Activate`
  (params (StartLocation :type "Vector Structure") (StartRotation :type "Rotator Structure"))
  (bind _returnvalue (`KismetMaterialLibrary.CreateDynamicMaterialInstance` "/Game/T5_PuzzleGame/Art/Materials/MI_Outline.MI_Outline"))
  (`PrimitiveComponent.SetMaterial` (`self.StaticMesh`) 0 _returnvalue)
  (`PrimitiveComponent.SetRenderCustomDepth` (`self.StaticMesh`) true)
  (`PrimitiveComponent.SetCustomDepthStencilValue` (`self.StaticMesh`) 1)
  (`self.K2_SetActorRotation` StartRotation)
  (bind _output_get (set `self.StartPosition` StartLocation))
  (set `self.EndPosition` (+ _output_get (* (`self.GetActorUpVector`) 50.0)))
  (`SceneComponent.SetVisibility` (`self.StaticMesh`) true false)
  (bind (_direction _alpha) (`Timeline|Timeline_0` :!label _label)
    (:`Update`
      (`self.K2_SetActorLocation` (`KismetMathLibrary.VLerp` (`self.StartPosition`) (`self.EndPosition`) _alpha)))))

(event `Deactivate`
  (`SceneComponent.SetVisibility` (`self.StaticMesh`) false false)
  (goto _label :!via `Stop`))

(event `self.ReceiveBeginPlay`
  (`SceneComponent.SetVisibility` (`self.StaticMesh`) false false))

(fn `UserConstructionScript`)