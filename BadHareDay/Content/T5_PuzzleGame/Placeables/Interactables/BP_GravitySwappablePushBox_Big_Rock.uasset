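; Rock variant of the big gravity-swappable push box that disables its interaction collision while another big box sits on it.
; When CheckAbove is enabled, a looping timer line-traces along actor up from up to three start points.
; A big-box hit disables Collision, restores the default material and turns off custom depth.
; Otherwise Collision returns to query-only; the traces draw debug lines.
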(event `self.ReceiveBeginPlay`
  ;[1 1 1] Start Timer
  (`parent.ReceiveBeginPlay`)
  (if (`self.bCheckAbove`)
    (`KismetSystemLibrary.K2_SetTimer` null "CheckAbove" 0.5 true)))

(event `CheckAbove`
  (bind _returnvalue (`SceneComponent.K2_GetComponentLocation` (`self.CheckAboveRayStartPos3`)))
  (bind _returnvalue_2 (`SceneComponent.K2_GetComponentLocation` (`self.CheckAboveRayStartPos1`)))
  (bind _returnvalue_3 (`SceneComponent.K2_GetComponentLocation` (`self.CheckAboveRayStartPos2`)))
  ;[1 1 1] Ray from CheckAboveRayStartPos1
  (bind (_outhit _returnvalue_4) (`KismetSystemLibrary.LineTraceSingleForObjects` :`Start` _returnvalue_2 :`End` (+ _returnvalue_2 (* (`self.GetActorUpVector`) (`self.CheckAboveLineLength`))) :`ObjectTypes` (`self.WhatToDetect`) :`DrawDebugType` "ForDuration" :`DrawTime` 1.0))
  (if _returnvalue_4
    (cast `/Game/T5_PuzzleGame/Placeables/Interactables/BP_GravitySwappablePushBox_Big` (`.HitActor` (`GameplayStatics.BreakHitResult` _outhit))
      (:`then`
        (`PrimitiveComponent.SetCollisionEnabled` (`self.Collision`) "NoCollision")
        (`PrimitiveComponent.SetMaterial` (`self.StaticMesh`) 0 (`self.DefaultMat`))
        (`PrimitiveComponent.SetRenderCustomDepth` (`self.StaticMesh`) false))
      (:`CastFailed`
        ;[1 1 1] Ray from CheckAboveRayStartPos2
        (bind (_outhit_2 _returnvalue_5) (`KismetSystemLibrary.LineTraceSingleForObjects` :`Start` _returnvalue_3 :`End` (+ _returnvalue_3 (* (`self.GetActorUpVector`) (`self.CheckAboveLineLength`))) :`ObjectTypes` (`self.WhatToDetect`) :`DrawDebugType` "ForDuration" :`DrawTime` 1.0 :!label _label))
        (if _returnvalue_5
          (cast `/Game/T5_PuzzleGame/Placeables/Interactables/BP_GravitySwappablePushBox_Big` (`.HitActor` (`GameplayStatics.BreakHitResult` _outhit_2))
            (:`then`
              (`PrimitiveComponent.SetCollisionEnabled` (`self.Collision`) "NoCollision")
              (`PrimitiveComponent.SetMaterial` (`self.StaticMesh`) 0 (`self.DefaultMat`))
              (`PrimitiveComponent.SetRenderCustomDepth` (`self.StaticMesh`) false))
            (:`CastFailed`
              ;[1 1 1] Ray from CheckAboveRayStartPos3
              (bind (_outhit_3 _returnvalue_6) (`KismetSystemLibrary.LineTraceSingleForObjects` :`Start` _returnvalue :`End` (+ _returnvalue (* (`self.GetActorUpVector`) (`self.CheckAboveLineLength`))) :`ObjectTypes` (`self.WhatToDetect`) :`DrawDebugType` "ForDuration" :`DrawTime` 1.0 :!label _label_2))
              (if _returnvalue_6
                (cast `/Game/T5_PuzzleGame/Placeables/Interactables/BP_GravitySwappablePushBox_Big` (`.HitActor` (`GameplayStatics.BreakHitResult` _outhit_3))
                  (:`then`
                    (`PrimitiveComponent.SetCollisionEnabled` (`self.Collision`) "NoCollision")
                    (`PrimitiveComponent.SetMaterial` (`self.StaticMesh`) 0 (`self.DefaultMat`))
                    (`PrimitiveComponent.SetRenderCustomDepth` (`self.StaticMesh`) false))
                  (:`CastFailed`
                    (`PrimitiveComponent.SetCollisionEnabled` (`self.Collision`) "QueryOnly" :!label _label_3)))
                (else
                  (goto _label_3)))))
          (else
            (goto _label_2)))))
    (else
      (goto _label))))

(fn `UserConstructionScript`
  (`parent.UserConstructionScript`))