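; BP_SectionBlocker is a placeable puzzle-game actor that moves itself to close off a section once the player enters its trigger.
; On BeginPlay it caches the root's world location as the start and the End component's location as the target.
; The first Box overlap by a BP_Player passes a DoOnce and calls CloseSection, where a timeline lerps the root between those points without sweeping.
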(event `CloseSection`
  (bind (_direction _alpha) (`Timeline|Timeline_0` :!via `PlayFromStart`)
    (:`Update`
      (`SceneComponent.K2_SetWorldLocation` (`self.DefaultSceneRoot`) (`KismetMathLibrary.VLerp` (`self.StartLocation`) (`self.EndLocation`) _alpha) false false))))

(event `self.ReceiveBeginPlay`
  (set `self.StartLocation` (`SceneComponent.K2_GetComponentLocation` (`self.DefaultSceneRoot`)))
  (set `self.EndLocation` (`SceneComponent.K2_GetComponentLocation` (`self.End`))))

(event `self.Box.OnComponentBeginOverlap`
  (params (OverlappedComponent :type "PrimitiveComponent Object Reference") (OtherActor :type "Actor Object Reference") (OtherComp :type "PrimitiveComponent Object Reference") (OtherBodyIndex :type Integer) (bFromSweep :type Boolean) (SweepResult :type "HitResult Structure (by ref)"))
  (if (== (`GameplayStatics.GetObjectClass` OtherActor) "/Game/T5_PuzzleGame/Characters/BP_Player.BP_Player_C")
    (`/Engine/EditorBlueprintResources/StandardMacros.DoOnce` false
      (:`Completed`
        (`self.CloseSection`)))))

(fn `UserConstructionScript`)