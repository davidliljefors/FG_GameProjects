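; Player character for a gravity-flip puzzle game, handling checkpoints, death and respawn, relic unlocks and Level1 tutorial popups.
; Gravity flips stop movement, briefly block input and release grabbed boxes, while highlight events toggle an arrow child actor.
; Death, triggerable by sustained head-hitbox overlap, dissolves the mesh via timeline, then restores checkpoint location and gravity.
; Collectible counts unlock two relic powers, updating the relic HUD and opening an ability popup.
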(event `Key|Escape`
  (params (Key :type "Key Structure"))
  (:`Pressed`
    (`GameplayStatics.OpenLevel` "MainMenu_New")))

(event `self.ReceiveHit`
  (params (MyComp :type "PrimitiveComponent Object Reference") (Other :type "Actor Object Reference") (OtherComp :type "PrimitiveComponent Object Reference") (bSelfMoved :type Boolean) (HitLocation :type "Vector Structure") (HitNormal :type "Vector Structure") (NormalImpulse :type "Vector Structure") (Hit :type "HitResult Structure (by ref)"))
  (`/Engine/EditorBlueprintResources/StandardMacros.DoOnce` false :!label _label
    (:`Completed`
      (`self.EnableInput` (`GameplayStatics.GetPlayerController` 0) :!label _label_2))))

(event `OnFlipGravity_Event_0`
  (params (bInverted :type Boolean))
  (set `MovementComponent.Velocity` (0.0 0.0 0.0) (`self.CharacterMovement`))
  (`self.DisableInput` (`GameplayStatics.GetPlayerController` 0))
  (`|ExecutionSequence`
    (:`then_0`
      (goto _label :!via `Reset`))
    (:`then_1`
      (`KismetSystemLibrary.Delay` 1.5)
      (goto _label_2))))

(event `self.CapsuleComponent.OnComponentHit`
  (params (HitComponent :type "PrimitiveComponent Object Reference") (OtherActor :type "Actor Object Reference") (OtherComp :type "PrimitiveComponent Object Reference") (NormalImpulse :type "Vector Structure") (Hit :type "HitResult Structure (by ref)")))

(event `self.ReceiveBeginPlay`
  (`parent.ReceiveBeginPlay`)
  (add `self.OnCheckPointEnter` (delegate `CheckPointEnter`))
  (`self.FadeInPlayer`)
  (bind _asbp_arrow (cast `/Game/T5_PuzzleGame/Placeables/Interactables/BP_Arrow` (`ChildActorComponent.ChildActor` (`self.GravArrow`))))
  (set `self.Arrow` _asbp_arrow)
  (add `ClickInteractComponent.OnActivateHighlight` (`self.ClickInteract`) (delegate `Highlight`))
  (add `GravitySwapComponent.OnFlipGravity` (`self.GravitySwap`) (delegate `OnFlipGravity_Event_0`))
  (`/Engine/EditorBlueprintResources/StandardMacros.IsValid` (`self.RelicGUIVar`)
    (:`Is Not Valid`
      (bind _returnvalue (`|CreateWidget` "/Game/T5_PuzzleGame/UserInterfaces/WBP_Relics.WBP_Relics_C"))
      (bind _output_get (set `self.RelicGUIVar` _returnvalue))
      (`UserWidget.AddToViewport` _output_get 0)
      (bind _returnvalue_2 (`GameplayStatics.GetActorOfClass` "/Game/T5_PuzzleGame/Placeables/CheckpointSystem/BP_RespawnManger.BP_RespawnManger_C"))
      (set `self.RespawnManager` _returnvalue_2))))

(event `Highlight`
  (params (HightlightType :type "EOutlineType Enum" :default "None"))
  (bind _arrow (`self.Arrow`))
  (switch `EOutlineType` HightlightType
    (:`None`
      (`/Game/T5_PuzzleGame/Placeables/Interactables/BP_Arrow.Deactivate` _arrow :!label _label_3))
    (:`Hover`
      (`/Game/T5_PuzzleGame/Placeables/Interactables/BP_Arrow.Activate` _arrow (`SceneComponent.K2_GetComponentLocation` (`self.GravArrow`)) (`self.K2_GetActorRotation` (`self.Arrow`)) :!label _label_4))
    (:`Selected`
      (goto _label_4))
    (:`Swappable`
      (goto _label_4))
    (:`NonSwappable`
      (goto _label_3))))

(event `CheckPointEnter`
  (set `self.SavedFlipGravity` (`GravitySwapComponent.bFlipGravity` (`self.GravitySwap`)))
  (set `self.SavedLocation` (`self.K2_GetActorLocation`)))

(event `CheckPointInterface.OnRest`
  (`GravitySwappable.SetFlipGravity` (`self.GravitySwap`) (`self.FlipGravitySave`))
  (`CheckPointInterface.OnRest` (`self.BP_DeathTriggerComponent`))
  (set `MovementComponent.Velocity` (0.0 0.0 0.0) (`self.CharacterMovement`)))

(event `CheckPointInterface.OnEnterCheckPoint`
  (params (ActorCaller :type "Actor Object Reference") (CheckpointCaller :type "Actor Object Reference"))
  (set `self.FlipGravitySave` (`GravitySwapComponent.bFlipGravity` (`self.GravitySwap`))))

(event `Key|LeftShift`
  (params (Key :type "Key Structure"))
  (:`Pressed`
    (bind _outactors (`GameplayStatics.GetAllActorsOfClass` "/Game/T5_PuzzleGame/BP_FollowCamera.BP_FollowCamera_C"))
    (`/Game/T5_PuzzleGame/BP_FollowCamera.ZoomedView` (`|GetArrayItem` _outactors)))
  (:`Released`
    (bind _outactors_2 (`GameplayStatics.GetAllActorsOfClass` "/Game/T5_PuzzleGame/BP_FollowCamera.BP_FollowCamera_C"))
    (`/Game/T5_PuzzleGame/BP_FollowCamera.NormalVieqw` (`|GetArrayItem` _outactors_2))))

(event `self.OnJumped`
  (bind _currentgrabbingbox (`self.CurrentGrabbingBox`))
  ;[1 1 1] Release Grab if grabbing
  (`/Engine/EditorBlueprintResources/StandardMacros.IsValid` _currentgrabbingbox :!label _label_5
    (:`Is Valid`
      (`/Game/T5_PuzzleGame/Core/BP_ApproachGrabComponent.Release` (`self.GetComponentByClass` (`ActorComponent.GetOwner` _currentgrabbingbox) "/Game/T5_PuzzleGame/Core/BP_ApproachGrabComponent.BP_ApproachGrabComponent_C")))))

(event `self.GravitySwap.OnFlipGravity`
  (params (bInverted :type Boolean))
  (goto _label_5))

(event `self.OnCollectibleAdded`
  (params (Type :type "ECollectibleType Enum" :default "Coin") (NewCount :type Integer))
  ;[1 1 1] OnCollectible added
  (bind _output_get (set `self.CurrentRelicCount` NewCount))
  (`KismetSystemLibrary.PrintString` (`KismetStringLibrary.Concat_StrStr` "Current Relic Count: " (`KismetStringLibrary.Conv_IntToString` _output_get)))
  (`|ExecutionSequence`
    (:`then_0`
      ;[1 1 1] Unlock Relic 1 power
      (if (>= NewCount (`self.Relic1ToUnlockPower`))
        (if (not (`self.bHasRelic1`))
          (set `self.bHasRelic1` true)
          (`KismetSystemLibrary.PrintString` "Player unlocked relic 1 full power" true true (struct :`R` 1.0 :`G` 0.580408 :`A` 1.0))
          (`/Game/T5_PuzzleGame/UserInterfaces/WBP_Relics.Ability 1` (`self.RelicGUIVar`))
          (`/Engine/EditorBlueprintResources/StandardMacros.DoOnce` false
            (:`Completed`
              (`self.AbilityGained` :!label _label_6))))))
    (:`then_1`
      ;[1 1 1] Unlock Relic 2 power
      (if (>= NewCount (`self.Relic2ToUnlockPower`))
        (if (not (`self.bHasRelic2`))
          (set `self.bHasRelic2` true)
          (`KismetSystemLibrary.PrintString` "Player unlocked relic 2 full power" true true (struct :`R` 1.0 :`G` 0.580408 :`A` 1.0))
          (`/Game/T5_PuzzleGame/UserInterfaces/WBP_Relics.Ability 2` (`self.RelicGUIVar`))
          (`/Engine/EditorBlueprintResources/StandardMacros.DoOnce` false
            (:`Completed`
              (goto _label_6))))))))

(event `AbilityGained`
  (bind _returnvalue (`GameplayStatics.GetPlayerController` 0))
  ;[1 1 1] Show Ability Popup
  (bind _returnvalue_2 (`|CreateWidget` "/Game/T5_PuzzleGame/UserInterfaces/WBP_AbilityPopup.WBP_AbilityPopup_C" _returnvalue))
  (`UserWidget.AddToViewport` _returnvalue_2 0)
  (`WidgetBlueprintLibrary.SetInputMode_UIOnlyEx` _returnvalue null)
  (`ActorComponent.Deactivate` (`self.CharacterMovement`))
  (`NavMovementComponent.StopActiveMovement` (`self.CharacterMovement`)))

(event `self.HeadSmashHitbox.OnComponentBeginOverlap`
  (params (OverlappedComponent :type "PrimitiveComponent Object Reference") (OtherActor :type "Actor Object Reference") (OtherComp :type "PrimitiveComponent Object Reference") (OtherBodyIndex :type Integer) (bFromSweep :type Boolean) (SweepResult :type "HitResult Structure (by ref)"))
  (`|ExecutionSequence`
    (:`then_0`
      (goto _label_7 :!via `Open`))
    (:`then_1`
      (`KismetSystemLibrary.RetriggerableDelay` 0.5)
      (`/Engine/EditorBlueprintResources/StandardMacros.Gate` true :!label _label_7
        (:`Exit`
          (`self.Die`))))
    (:`then_2`
      (`KismetSystemLibrary.PrintString` "hit head"))))

(event `self.HeadSmashHitbox.OnComponentEndOverlap`
  (params (OverlappedComponent :type "PrimitiveComponent Object Reference") (OtherActor :type "Actor Object Reference") (OtherComp :type "PrimitiveComponent Object Reference") (OtherBodyIndex :type Integer))
  (goto _label_7 :!via `Close`))

(event `FirstThorns`
  (bind _returnvalue (`GameplayStatics.GetCurrentLevelName` true))
  (if (`KismetStringLibrary.EqualEqual_StrStr` _returnvalue "Level1")
    (`/Engine/EditorBlueprintResources/StandardMacros.DoOnce` false
      (:`Completed`
        (bind _returnvalue_2 (`|CreateWidget` "/Game/T5_PuzzleGame/UserInterfaces/WPB_TutorialText.WPB_TutorialText_C"))
        (set `/Game/T5_PuzzleGame/UserInterfaces/WPB_TutorialText.Select Tutorial` "NewEnumerator7" _returnvalue_2)
        (`UserWidget.AddToViewport` _returnvalue_2 0)
        (bind (_direction _newtrack_0) (`Timeline|Timeline_0`)
          (:`Update`
            (`Widget.SetRenderOpacity` _returnvalue_2 _newtrack_0))
          (:`Finished`
            (`KismetSystemLibrary.Delay` 3.0)
            (bind (_direction_2 _newtrack_0_2) (`Timeline|Timeline_1`)
              (:`Update`
                (`Widget.SetRenderOpacity` _returnvalue_2 _newtrack_0_2))
              (:`Finished`
                (`Widget.RemoveFromParent` _returnvalue_2)))))))))

(event `FirstCrushed`
  (bind _returnvalue (`GameplayStatics.GetCurrentLevelName` true))
  (if (`KismetStringLibrary.EqualEqual_StrStr` _returnvalue "Level1")
    (`/Engine/EditorBlueprintResources/StandardMacros.DoOnce` false
      (:`Completed`
        (bind _returnvalue_2 (`|CreateWidget` "/Game/T5_PuzzleGame/UserInterfaces/WPB_TutorialText.WPB_TutorialText_C"))
        (set `/Game/T5_PuzzleGame/UserInterfaces/WPB_TutorialText.Select Tutorial` "NewEnumerator8" _returnvalue_2)
        (`UserWidget.AddToViewport` _returnvalue_2 0)
        (bind (_direction _newtrack_0) (`Timeline|Timeline_2`)
          (:`Update`
            (`Widget.SetRenderOpacity` _returnvalue_2 _newtrack_0))
          (:`Finished`
            (`KismetSystemLibrary.Delay` 3.0)
            (bind (_direction_2 _newtrack_0_2) (`Timeline|Timeline_3`)
              (:`Update`
                (`Widget.SetRenderOpacity` _returnvalue_2 _newtrack_0_2))
              (:`Finished`
                (`Widget.RemoveFromParent` _returnvalue_2)))))))))

(event `Die`
  ;[1 1 1] Death and Respawn
  (`/Engine/EditorBlueprintResources/StandardMacros.DoOnce` false :!label _label_8
    (:`Completed`
      (set `self.IsDead` true)
      (`self.DoDissolveEffect`)
      (`GameplayStatics.PlaySound2D` "/Game/T5_PuzzleGame/Audio/CUE_Death.CUE_Death" 1.0 1.0 0.0 null null)
      (`PrimitiveComponent.SetCollisionEnabled` (`self.CapsuleComponent`) "NoCollision")
      (`ActorComponent.SetComponentTickEnabled` (`self.CharacterMovement`) false)
      (`KismetSystemLibrary.Delay` (`self.RespawnDelay`))
      (`self.OnRespawn`))))

(event `ResetDeath`
  ;[1 1 1] Death and Respawn
  (goto _label_8 :!via `Reset`))

(event `OnRespawn`
  (bind _savedflipgravity (`self.SavedFlipGravity`))
  ;[1 1 1] Death and Respawn
  (`PrimitiveComponent.SetCollisionEnabled` (`self.CapsuleComponent`) "QueryAndPhysics")
  (`ActorComponent.SetComponentTickEnabled` (`self.CharacterMovement`) true)
  (set `self.IsDead` false)
  (`self.ResetDissolve`)
  (`self.ResetDeath`)
  (`self.OnPlayerRespawn`)
  (`self.K2_SetActorLocation` (`self.SavedLocation`) false true)
  (set `self.bFlipGravity` _savedflipgravity)
  (set `GravitySwapComponent.bFlipGravity` _savedflipgravity (`self.GravitySwap`))
  (`MovementComponent.StopMovementImmediately` (`self.CharacterMovement`)))

(event `FadeInPlayer`
  (bind (_direction _dissolveamount _tiling _cutoff) (`Timeline|Timeline_4` :!via `PlayFromStart`)
    (:`Update`
      (`self.DisableInput` (`GameplayStatics.GetPlayerController` 0))
      (`MeshComponent.SetScalarParameterValueOnMaterials` (`self.Mesh`) "DissolveAmount" _dissolveamount)
      (`MeshComponent.SetScalarParameterValueOnMaterials` (`self.Mesh`) "Tiling" _tiling)
      (`MeshComponent.SetScalarParameterValueOnMaterials` (`self.Mesh`) "Cutoff" _cutoff))
    (:`Finished`
      (`self.EnableInput` (`GameplayStatics.GetPlayerController` 0)))))

(event `DoDissolveEffect`
  (bind (_direction _dissolveamount _tiling) (`Timeline|DissolveEffect` :!via `PlayFromStart` :!label _label_9)
    (:`Update`
      (`MeshComponent.SetScalarParameterValueOnMaterials` (`self.Mesh`) "DissolveAmount" _dissolveamount)
      (`MeshComponent.SetScalarParameterValueOnMaterials` (`self.Mesh`) "Tiling" _tiling))))

(event `ResetDissolve`
  (`|ExecutionSequence`
    (:`then_0`
      (goto _label_9 :!via `Stop`))
    (:`then_1`
      (`MeshComponent.SetScalarParameterValueOnMaterials` (`self.Mesh`) "DissolveAmount" 10.0)
      (`MeshComponent.SetScalarParameterValueOnMaterials` (`self.Mesh`) "Tiling" 0.0))))

(fn `Add Relic`
  (params (Count :type Integer))
  (`KismetSystemLibrary.PrintString` "Player found a relic1 part" true true (struct :`R` 0.697199 :`G` 1.0 :`B` 0.865935 :`A` 1.0))
  (if (>= Count (`self.Relic1ToUnlockPower`))
    (set `self.bHasRelic1` true)
    (`KismetSystemLibrary.PrintString` "Player unlocked relic 1 full power" true true (struct :`R` 1.0 :`G` 0.580408 :`A` 1.0))
    (return)
    (else
      (return))))

(fn `UserConstructionScript`
  (`parent.UserConstructionScript`))