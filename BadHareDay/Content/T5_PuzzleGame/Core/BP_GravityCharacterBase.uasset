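; Base character for a gravity-swapping puzzle game, with a starting gravity and click-interaction highlights.
; When the GravitySwap component flips gravity, the camera boom's socket offset is negated to refocus the view.
; ClickInteract highlight events switch the mesh to an outline material and set a custom depth stencil per state, restoring the default material on None.
; Swap results are debug-printed, and a same-gravity failure spawns tutorial text at the player pawn.
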(event `self.ReceiveBeginPlay`
  (`self.SetGravityTarget` (`self.StartGravity`))
  (set `self.CameraBoomDefaultOffset` (`SpringArmComponent.SocketOffset` (`self.CameraBoom`)))
  (set `self.DefaultMat` (`PrimitiveComponent.GetMaterial` (`self.Mesh`) 0)))

(event `self.GravitySwap.OnFlipGravity`
  (params (bInverted :type Boolean))
  (bind _cameraboom (`self.CameraBoom`))
  (bind _cameraboomdefaultoffset (`self.CameraBoomDefaultOffset`))
  ;[1 1 1] On Flip Gravity :  Change camera focus when gravity flips
  (bind _output_get (set `self.bFlipGravity` bInverted))
  (if _output_get
    (set `SpringArmComponent.SocketOffset` (* _cameraboomdefaultoffset -1.0) _cameraboom)
    (else
      (set `SpringArmComponent.SocketOffset` _cameraboomdefaultoffset _cameraboom))))

(event `self.ClickInteract.OnActivateHighlight`
  (params (HightlightType :type "EOutlineType Enum" :default "None"))
  (bind _mesh (`self.Mesh`))
  ;[1 1 1] Show highlight
  (`PrimitiveComponent.SetMaterial` (`self.Mesh`) 0 (`self.OutlineMat`))
  (`PrimitiveComponent.SetRenderCustomDepth` (`self.Mesh`) true)
  (switch `EOutlineType` HightlightType
    (:`None`
      (`PrimitiveComponent.SetMaterial` (`self.Mesh`) 0 (`self.DefaultMat`))
      (`PrimitiveComponent.SetRenderCustomDepth` (`self.Mesh`) false))
    (:`Hover`
      (`PrimitiveComponent.SetCustomDepthStencilValue` _mesh 0))
    (:`Selected`
      (`PrimitiveComponent.SetCustomDepthStencilValue` _mesh 1))
    (:`Swappable`
      (`PrimitiveComponent.SetCustomDepthStencilValue` _mesh 2))
    (:`NonSwappable`
      (`PrimitiveComponent.SetCustomDepthStencilValue` _mesh 3))))

(event `self.ClickInteract.OnTrySwappingGravity`
  (params (SwapResult :type "ESwapResult Enum" :default "Success"))
  ;[1 1 1] Get Swap result
  (`KismetSystemLibrary.PrintString` (`|GetEnumeratorNameAsString` SwapResult))
  (switch `ESwapResult` SwapResult
    (:`Fail_SameGravity`
      (`|SpawnActorFromClass` "/Game/T5_PuzzleGame/Placeables/BP_TutorialText.BP_TutorialText_C" (`self.GetTransform` (`GameplayStatics.GetPlayerPawn` 0)) "Undefined" "OverrideRootScale" null "NewEnumerator5" null))))

(fn `UserConstructionScript`)