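; Base grabbable puzzle box whose gravity flips toward or away from the world origin, and which kills the player it falls onto.
; Physics runs only while grabbed or moving; velocity polling then freezes it as a solid obstacle.
; Release snaps it along a radial trace, gravity flips wake nearby boxes, and swappers pull it through by timeline.
; It also drives selection highlights and restores transform and gravity from checkpoints on respawn.
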(event `self.ClickInteract.OnClickInteract`)

(event `self.ClickInteract.OnResetClickInteract`)

(event `self.BP_ApproachGrabComponent.OnInteract`)

(event `self.BP_ApproachGrabComponent.OnInteractReleased`)

(event `self.ReceiveBeginPlay`
  (bind _bp_approachgrabcomponent (`self.BP_ApproachGrabComponent`))
  ;[1 1 1] BeginPlay
  (bind _asbp_player (cast `/Game/T5_PuzzleGame/Characters/BP_Player` (`GameplayStatics.GetPlayerCharacter` 0)))
  (bind _output_get (set `self.PlayerRef` _asbp_player))
  (add `/Game/T5_PuzzleGame/Characters/BP_Player.OnCheckPointEnter` _output_get (delegate `OnCheckPointEnter`))
  (add `/Game/T5_PuzzleGame/Characters/BP_Player.OnPlayerRespawn` _output_get (delegate `OnPlayerRespawn`))
  (add `/Game/T5_PuzzleGame/Core/BP_ApproachGrabComponent. OnGrabbed` _bp_approachgrabcomponent (delegate `Event OnGrabbed`))
  (add `/Game/T5_PuzzleGame/Core/BP_ApproachGrabComponent.OnReleased` _bp_approachgrabcomponent (delegate `Event OnReleased`))
  (set `self.DefaultMat` (`PrimitiveComponent.GetMaterial` (`self.StaticMesh`) 0))
  (`KismetSystemLibrary.Delay` 1.0)
  (if (not (`/Game/T5_PuzzleGame/Core/BP_ApproachGrabComponent.bIsGrabbed` (`self.BP_ApproachGrabComponent`)))
    (`self.BecomeStatic`)))

(event `Event OnGrabbed`
  (`self.BecomeActive`))

(event `OnCheckPointEnter`
  ;[1 1 1] OnCheckPointEnter
  (set `self.SavedTransform` (`self.GetTransform`))
  (set `self.SavedFlipGravity` (`GravitySwapComponent.bFlipGravity` (`self.GravitySwap`))))

(event `Event OnReleased`
  (if (== (`KismetArrayLibrary.Array_Length` (`PrimitiveComponent.GetOverlappingActors` (`self.StaticMesh`) "/Game/T5_PuzzleGame/Placeables/Interactables/BP_GravitySwapper.BP_GravitySwapper_C")) 0)
    (`/Engine/EditorBlueprintResources/StandardMacros.DoOnce` false :!label _label
      (:`Completed`
        (`KismetSystemLibrary.Delay` 0.05)
        (bind (_valid _location) (`self.GetPlaceLocation`))
        (if _valid
          (if (> (`KismetMathLibrary.Vector_DistanceSquared` _location (`self.K2_GetActorLocation`)) 5000.0)
            (set `self.LerpStartPos` (`self.K2_GetActorLocation`))
            (bind (_direction _t) (`Timeline|PlaceLerp` :!via `PlayFromStart` :!label _label_2)
              (:`Update`
                (bind (_sweephitresult _returnvalue) (`self.K2_SetActorLocation` (`KismetMathLibrary.VLerp` (`self.LerpStartPos`) _location _t) true))
                (if (not _returnvalue)
                  (`self.BecomeStatic`)
                  (`self.ResetPlace`)
                  (goto _label_2 :!via `Stop`)))
              (:`Finished`
                (`self.BecomeStatic` :!label _label_3)
                (`self.ResetPlace`)))
            (else
              (`self.K2_SetActorLocation` _location true)
              (goto _label_3))))))
    (else
      (`KismetSystemLibrary.Delay` 0.2) ; need some time for when pushed into swapper
      (`/Engine/EditorBlueprintResources/StandardMacros.Gate` false :!label _label_4
        (:`Exit`
          (if (`self.IsStationary` (`self.StaticMesh`)) :!label _label_5
            (`self.BecomeStatic`)
            (`self.OpenReleaseGate`)
            (else
              (`KismetSystemLibrary.Delay` 0.05)
              (goto _label_5))))))))

(event `ResetPlace`
  (goto _label :!via `Reset`))

(event `OnPlayerRespawn`
  ;[1 1 1] OnPlayerRespawn
  (`SceneComponent.K2_SetWorldTransform` (`self.StaticMesh`) (`self.SavedTransform`) false true)
  (set `GravitySwapComponent.bFlipGravity` (`self.SavedFlipGravity`) (`self.GravitySwap`)))

(event `OpenReleaseGate`
  (goto _label_4 :!via `Open`))

(event `CloseReleaseGate`
  (goto _label_4 :!via `Close`))

(event `OnBreakLayer`
  ;[1 1 1] On Flip Gravity
  (`|ExecutionSequence`
    (:`then_0`
      (goto _label_8 :!via `Close`))
    (:`then_1`
      (`KismetSystemLibrary.RetriggerableDelay` 1.0 :!label _label_6) ; Time for box to fall before checking if static
      (`|ExecutionSequence`
        (:`then_0`
          (goto _label_8 :!via `Open`))
        (:`then_1`
          (if (`self.IsStationary` (`self.StaticMesh`)) :!label _label_7
            (`/Engine/EditorBlueprintResources/StandardMacros.Gate` true :!label _label_8
              (:`Exit`
                (`self.BecomeStatic`)
                (`self.OpenReleaseGate`)))
            (else
              (`KismetSystemLibrary.Delay` 0.05)
              (goto _label_7))))))))

(event `self.GravitySwap.OnFlipGravity`
  (params (bInverted :type Boolean))
  ;[1 1 1] On Flip Gravity
  (`self.NotifyNearbyObjects`)
  (`GameplayStatics.PlaySound2D` "/Game/T5_PuzzleGame/Audio/GravitySwap_Cue.GravitySwap_Cue" 1.0 1.0 0.0 null null)
  (`self.CloseReleaseGate`)
  (`self.SetCollisionWithPlayer` false)
  (`PrimitiveComponent.SetSimulatePhysics` (`self.StaticMesh`) false)
  (`KismetSystemLibrary.Delay` (`self.FlipDelay`))
  (`self.BecomeActive`)
  (goto _label_6))

(event `self.ClickInteract.OnActivateHighlight`
  (params (HightlightType :type "EOutlineType Enum" :default "None"))
  (bind _staticmesh (`self.StaticMesh`))
  ;[1 1 1] Show highlight
  (`PrimitiveComponent.SetRenderCustomDepth` (`self.StaticMesh`) true)
  (switch `EOutlineType` HightlightType
    (:`None`
      (`PrimitiveComponent.SetMaterial` (`self.StaticMesh`) 0 (`self.DefaultMat`))
      (`PrimitiveComponent.SetRenderCustomDepth` (`self.StaticMesh`) false))
    (:`Hover`
      (`PrimitiveComponent.SetCustomDepthStencilValue` _staticmesh 0))
    (:`Selected`
      (`PrimitiveComponent.SetCustomDepthStencilValue` _staticmesh 1)
      (`GameplayStatics.PlaySound2D` "/Game/T5_PuzzleGame/Audio/GravitySelect_Cue.GravitySelect_Cue" 1.0 1.0 0.0 null null))
    (:`Swappable`
      (`PrimitiveComponent.SetCustomDepthStencilValue` _staticmesh 2))
    (:`NonSwappable`
      (`PrimitiveComponent.SetCustomDepthStencilValue` _staticmesh 3))))

(event `self.ClickInteract.OnTrySwappingGravity`
  (params (SwapResult :type "ESwapResult Enum" :default "Success"))
  ;[1 1 1] Get Swap result
  (`KismetSystemLibrary.PrintString` (`|GetEnumeratorNameAsString` SwapResult))
  (switch `ESwapResult` SwapResult
    (:`Fail_SameGravity`
      (`|SpawnActorFromClass` "/Game/T5_PuzzleGame/Placeables/BP_TutorialText.BP_TutorialText_C" (`self.GetTransform` (`GameplayStatics.GetPlayerPawn` 0)) "Undefined" "OverrideRootScale" null "NewEnumerator5" null))))

(event `self.StaticMesh.OnComponentBeginOverlap`
  (params (OverlappedComponent :type "PrimitiveComponent Object Reference") (OtherActor :type "Actor Object Reference") (OtherComp :type "PrimitiveComponent Object Reference") (OtherBodyIndex :type Integer) (bFromSweep :type Boolean) (SweepResult :type "HitResult Structure (by ref)"))
  ;[1 1 1] OnCollisionEnter, squash player?
  (if (and (`KismetMathLibrary.ClassIsChildOf` (`GameplayStatics.GetObjectClass` OtherActor) "/Script/GP2_Team5.GravityCharacter") (== (`GameplayStatics.GetObjectClass` OtherComp) "/Script/Engine.CapsuleComponent"))
    (bind _asbp_player (cast `/Game/T5_PuzzleGame/Characters/BP_Player` OtherActor))
    (if (`self.IsFallingOntoPlayer` _asbp_player)
      (`/Game/T5_PuzzleGame/Characters/BP_Player.Die` _asbp_player))))

(event `OnNearbyUpdated`
  ;[1 1 1] When nearby objects change gravity we might need to update ourselves
  (if (`self.IsStationary` (`self.StaticMesh`))
    (`self.BecomeActive`)
    (`KismetSystemLibrary.Delay` 0.25)
    (if (`self.IsStationary` (`self.StaticMesh`)) :!label _label_9
      (`self.BecomeStatic`)
      (else
        (`KismetSystemLibrary.Delay` 0.05)
        (goto _label_9)))))

(event `LerpGravitySwitch`
  (params (TargetPos :type "Vector Structure") (ActorToIgnore :type "Actor Object Reference"))
  (bind _returnvalue (`KismetMathLibrary.Normal` TargetPos))
  (bind _gravityswap (`self.GravitySwap`))
  ;[1 1 1] Lerp Position to gravity swapper
  (`self.CloseReleaseGate`)
  (`self.SetCollisionWithPlayer` false)
  (`PrimitiveComponent.SetCollisionEnabled` (`self.StaticMesh`) "PhysicsOnly")
  (set `self.LerpStartPos` (`self.K2_GetActorLocation`))
  (if (`GravitySwappable.GetFlipGravity` (`self.GravitySwap`))
    (set `self.LerpTargetPos` (+ TargetPos (* _returnvalue -200.0)))
    (bind (_direction _t) (`Timeline|GravitySwapperLerp` :!via `PlayFromStart` :!label _label_10)
      (:`Update`
        (`self.K2_SetActorLocation` (`KismetMathLibrary.VLerp` (`self.LerpStartPos`) (`self.LerpTargetPos`) _t) false true))
      (:`Finished`
        (`GravitySwappable.SetFlipGravity` _gravityswap (not (`GravitySwapComponent.bFlipGravity` _gravityswap)))
        (`KismetSystemLibrary.Delay` 0.5)
        (`PrimitiveComponent.SetCollisionEnabled` (`self.StaticMesh`) "QueryAndPhysics")))
    (else
      (set `self.LerpTargetPos` (+ TargetPos (* _returnvalue 25.0)))
      (goto _label_10 :!via `PlayFromStart`))))

(fn `BecomeActive`
  (bind _staticmesh (`self.StaticMesh`))
  (`PrimitiveComponent.SetSimulatePhysics` _staticmesh true)
  (`PrimitiveComponent.SetPhysicsLinearVelocity` _staticmesh (0.0 0.0 0.0) false "None")
  (return))

(fn `BecomeStatic`
  (`PrimitiveComponent.SetSimulatePhysics` (`self.StaticMesh`) false)
  (`self.SetCollisionWithPlayer` true)
  (`KismetSystemLibrary.PrintString` (`KismetStringLibrary.Concat_StrStr` (`KismetSystemLibrary.GetDisplayName` self) "became static"))
  (return))

(fn `GetPlaceLocation`
  (returns (Valid :type Boolean) (Location :type "Vector Structure"))
  (locals (TraceEnd :type "Vector Structure" :default (0.0 0.0 0.0)))
  (bind _returnvalue (`self.K2_GetActorLocation`))
  (if (`GravitySwapComponent.bFlipGravity` (`self.GravitySwap`))
    (set `local.TraceEnd` (* _returnvalue 2.0))
    (else
      (set `local.TraceEnd` (* _returnvalue 0.0))))
  (bind (_outhit _returnvalue_2) (`KismetSystemLibrary.LineTraceSingle` :`Start` (`self.K2_GetActorLocation`) :`End` (`local.TraceEnd`) :`TraceChannel` "TraceTypeQuery1" :`bTraceComplex` true :`DrawDebugType` "ForDuration" :`DrawTime` 3.0))
  (if _returnvalue_2
    (if (`GravitySwapComponent.bFlipGravity` (`self.GravitySwap`))
      (bind (_bblockinghit _binitialoverlap _time _distance _location) (`GameplayStatics.BreakHitResult` _outhit))
      (return true (- _location (* (`KismetMathLibrary.Normal` _location) (`self.StaticMeshHeight`))))
      (else
        (return true _location)))
    (else
      (return true (0.0 0.0 0.0)))))

(fn `IsFallingOntoPlayer`
  (params (Player :type "GravityCharacter Object Reference"))
  (returns (Value :type Boolean))
  (locals (SquaredVelocityToKill :type "Float (double-precision)" :default 100.0))
  ;[1 1 1] Is Box velocity going in the same direction as box->player, and is it going fast enough
  (if (`SceneComponent.IsSimulatingPhysics` (`self.StaticMesh`) "None")
    (bind _returnvalue (`PrimitiveComponent.GetPhysicsLinearVelocity` (`self.StaticMesh`) "None"))
    (if (> (`KismetMathLibrary.VSizeSquared` _returnvalue) (`local.SquaredVelocityToKill`))
      (if (> (`KismetMathLibrary.Dot_VectorVector` _returnvalue (`KismetMathLibrary.GetDirectionUnitVector` (`self.K2_GetActorLocation`) (`self.K2_GetActorLocation` Player))) 0.0)
        (return true)
        (else
          _)))
    (return false)
    (else
      (return false))))

(fn `IsStationary`
  (params (`Physics Comp` :type "PrimitiveComponent Object Reference"))
  (returns (value :type Boolean))
  (bind _returnvalue (`PrimitiveComponent.GetPhysicsLinearVelocity` `Physics Comp` "None"))
  (return (< (`KismetMathLibrary.VSizeSquared` _returnvalue) 5.0)))

(fn `NotifyNearbyObjects`
  (bind (_outactors _returnvalue) (`KismetSystemLibrary.SphereOverlapActors` (`self.K2_GetActorLocation`) 100.0 (`|MakeArray` "ObjectTypeQuery10" "ObjectTypeQuery12" :!type "EObjectTypeQuery Enum") "BP_GravitySwappablePushBoxBase_C" (`|MakeArray` self :!type "Actor Object Reference")))
  (if _returnvalue
    (for _array_element _outactors
      (bind _asbp_gravity_swappable_push_box_base (cast `/Game/T5_PuzzleGame/Core/BP_GravitySwappablePushBoxBase` _array_element))
      (`self.OnNearbyUpdated` _asbp_gravity_swappable_push_box_base))))

(fn `Set Grond Collision`
  (params (CollisionEnabled :type "ECollisionResponse Enum" :default "ECR_Ignore"))
  (`PrimitiveComponent.SetCollisionResponseToChannel` (`self.Capsule`) "ECC_GameTraceChannel2" CollisionEnabled)
  (`PrimitiveComponent.SetCollisionResponseToChannel` (`self.Capsule1`) "ECC_GameTraceChannel2" CollisionEnabled)
  (`PrimitiveComponent.SetCollisionResponseToChannel` (`self.Capsule3`) "ECC_GameTraceChannel2" CollisionEnabled)
  (`PrimitiveComponent.SetCollisionResponseToChannel` (`self.Capsule2`) "ECC_GameTraceChannel2" CollisionEnabled))

(fn `SetCollisionWithPlayer`
  (params (On :type Boolean))
  (if On
    (`PrimitiveComponent.SetCollisionResponseToChannel` (`self.StaticMesh`) "ECC_Pawn" "ECR_Block")
    (`PrimitiveComponent.SetCollisionResponseToChannel` (`self.StaticMesh`) "ECC_GameTraceChannel1" "ECR_Overlap")
    (else
      (`PrimitiveComponent.SetCollisionResponseToChannel` (`self.StaticMesh`) "ECC_Pawn" "ECR_Overlap")
      (`PrimitiveComponent.SetCollisionResponseToChannel` (`self.StaticMesh`) "ECC_GameTraceChannel1" "ECR_Ignore")))
  (return))

(fn `SetRotationFromGround`
  (`self.K2_SetActorRotation` (`KismetMathLibrary.MakeRotationFromAxes` (-1.0 0.0 0.0) (`self.GetActorRightVector`) (`self.K2_GetActorLocation`)) true))

(fn `UserConstructionScript`)