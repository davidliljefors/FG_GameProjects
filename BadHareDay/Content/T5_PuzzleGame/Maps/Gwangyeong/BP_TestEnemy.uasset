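; Test enemy for a puzzle map that patrols along a spline and reacts to clicks and gravity flips.
; A Timeline drives position and rotation, resuming from a point estimated by distances to the spline's endpoints.
; Clicking toggles a point light and halts movement; resetting turns it off and resumes after a delay.
; Flipping gravity stops the Timeline, enables mesh physics and swaps between two splines.
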(event `self.ClickInteract.OnClickInteract`
  (bind _output_get (set `self.bLightOn` (not (`self.bLightOn`))))
  (`SceneComponent.SetVisibility` (`self.TempPointLight`) _output_get false)
  (set `self.bSelected` true)
  (`self.StopMove`))

(event `self.ClickInteract.OnResetClickInteract`
  (bind _output_get (set `self.bLightOn` false))
  (`SceneComponent.SetVisibility` (`self.TempPointLight`) _output_get false)
  (set `self.bSelected` false)
  (`KismetSystemLibrary.Delay` 2.0)
  (if (not (`TimelineComponent.IsPlaying` (`self.MoveTimeline`)))
    (`self.StartMove`)))

(event `self.ReceiveBeginPlay`
  (`SceneComponent.SetVisibility` (`self.TempPointLight`) (`self.bLightOn`) false)
  (`self.StartMove`))

(event `self.GravitySwap.OnFlipGravity`
  (params (bInverted :type Boolean))
  (`PrimitiveComponent.SetSimulatePhysics` (`self.StaticMesh`) true)
  (`self.SetActorTickEnabled` true)
  (`TimelineComponent.Stop` (`self.MoveTimeline`))
  (if (== (`self.CurrentSpline`) (`self.Spline1Ref`))
    (set `self.CurrentSpline` (`self.Spline0Ref`))
    (else
      (set `self.CurrentSpline` (`self.Spline1Ref`)))))

(event `StartMove`
  (bind _movetimeline (`self.MoveTimeline`))
  (bind _myyspline (`/Game/T5_PuzzleGame/Maps/Gwangyeong/BP_EnemySpline.MyySpline` (`self.CurrentSpline`)))
  (bind _returnvalue (`KismetMathLibrary.Vector_Distance` (`self.K2_GetActorLocation`) (`SplineComponent.GetLocationAtSplinePoint` (`/Game/T5_PuzzleGame/Maps/Gwangyeong/BP_EnemySpline.MyySpline` (`self.CurrentSpline`)) 0 "World")))
  (bind _returnvalue_2 (`KismetMathLibrary.Lerp` 0.0 (`SplineComponent.GetSplineLength` (`/Game/T5_PuzzleGame/Maps/Gwangyeong/BP_EnemySpline.MyySpline` (`self.CurrentSpline`))) (`self.Alpha`)))
  (`PrimitiveComponent.SetSimulatePhysics` (`self.StaticMesh`) false)
  (`self.SetActorTickEnabled` true)
  (`TimelineComponent.SetPlayRate` _movetimeline (`self.MoveSpeed`))
  (`TimelineComponent.SetNewTime` _movetimeline (/ _returnvalue (+ _returnvalue (`KismetMathLibrary.Vector_Distance` (`self.K2_GetActorLocation`) (`SplineComponent.GetLocationAtSplinePoint` _myyspline (`SplineComponent.GetNumberOfSplinePoints` _myyspline) "World")))))
  (bind (_direction _alpha) (`Timeline|MoveTimeline`)
    (:`Update`
      (set `self.Alpha` _alpha)
      (if (not (`self.bSelected`))
        (`self.K2_SetActorLocationAndRotation` (`SplineComponent.GetLocationAtDistanceAlongSpline` (`/Game/T5_PuzzleGame/Maps/Gwangyeong/BP_EnemySpline.MyySpline` (`self.CurrentSpline`)) _returnvalue_2 "World") (`SplineComponent.GetRotationAtDistanceAlongSpline` (`/Game/T5_PuzzleGame/Maps/Gwangyeong/BP_EnemySpline.MyySpline` (`self.CurrentSpline`)) _returnvalue_2 "World"))))))

(event `StopMove`
  (`self.SetActorTickEnabled` false)
  (`PrimitiveComponent.SetSimulatePhysics` (`self.StaticMesh`) false)
  (`TimelineComponent.Stop` (`self.MoveTimeline`)))

(fn `Set Grond Collision`
  (params (CollisionEnabled :type "ECollisionResponse Enum" :default "ECR_Ignore"))
  (`PrimitiveComponent.SetCollisionResponseToChannel` (`self.Capsule`) "ECC_GameTraceChannel2" CollisionEnabled)
  (`PrimitiveComponent.SetCollisionResponseToChannel` (`self.Capsule1`) "ECC_GameTraceChannel2" CollisionEnabled)
  (`PrimitiveComponent.SetCollisionResponseToChannel` (`self.Capsule3`) "ECC_GameTraceChannel2" CollisionEnabled)
  (`PrimitiveComponent.SetCollisionResponseToChannel` (`self.Capsule2`) "ECC_GameTraceChannel2" CollisionEnabled))

(fn `UserConstructionScript`)