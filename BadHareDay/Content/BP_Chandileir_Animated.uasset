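; Gravity-swappable chandelier on cables that moves between its placed location and EndPos when flipped, and can crush the player.
; Flipping starts a swept Tick lerp with an impact sound; player respawn restores the saved side.
; A kill capsule fitted from both endpoints kills an overlapping player after a delay on flip.
; Click highlights show an arrow along the world-origin radial axis, and hits on ClickBox stop gravity-swappable push boxes.
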(event `OnActivateHighlight_Event_0`
  (params (HightlightType :type "EOutlineType Enum" :default "None"))
  (bind _arrow1 (`self.Arrow1`))
  (switch `EOutlineType` HightlightType
    (:`None`
      (`/Game/T5_PuzzleGame/Placeables/Interactables/BP_Arrow.Deactivate` _arrow1 :!label _label))
    (:`Hover`
      (`/Game/T5_PuzzleGame/Placeables/Interactables/BP_Arrow.Activate` _arrow1 (select `bool` (`GravitySwapComponent.bFlipGravity` (`self.GravitySwap`)) :`false` (+ (`SceneComponent.K2_GetComponentLocation` (`self.StaticMesh`)) (* (`KismetMathLibrary.GetDirectionUnitVector` (0.0 0.0 0.0) (`SceneComponent.K2_GetComponentLocation` (`self.StaticMesh`))) 50.0)) :`true` (+ (`SceneComponent.K2_GetComponentLocation` (`self.StaticMesh`)) (* (`KismetMathLibrary.GetDirectionUnitVector` (`SceneComponent.K2_GetComponentLocation` (`self.StaticMesh`))) 50.0))) (select `bool` (`GravitySwapComponent.bFlipGravity` (`self.GravitySwap`)) :`false` (`KismetMathLibrary.MakeRotFromZ` (`KismetMathLibrary.GetDirectionUnitVector` (0.0 0.0 0.0) (`SceneComponent.K2_GetComponentLocation` (`self.StaticMesh`)))) :`true` (`KismetMathLibrary.MakeRotFromZ` (`KismetMathLibrary.GetDirectionUnitVector` (`SceneComponent.K2_GetComponentLocation` (`self.StaticMesh`))))) :!label _label_2))
    (:`Selected`
      (goto _label_2))
    (:`Swappable`
      (goto _label_2))
    (:`NonSwappable`
      (goto _label))))

(event `self.ReceiveBeginPlay`
  (`CableComponent.SetAttachEndTo` (`self.Cable1`) (`self.CableHinge`) "None" "None")
  (`CableComponent.SetAttachEndTo` (`self.Cable2`) (`self.CableHinge`) "None" "None")
  (`CableComponent.SetAttachEndTo` (`self.Cable3`) (`self.CableHinge`) "None" "None")
  (`CableComponent.SetAttachEndTo` (`self.Cable`) (`self.CableHinge`) "None" "None")
  (bind _asbp_player (cast `/Game/T5_PuzzleGame/Characters/BP_Player` (`GameplayStatics.GetPlayerCharacter` 0)))
  (bind _output_get (set `self.PlayerRef_0` _asbp_player))
  (add `/Game/T5_PuzzleGame/Characters/BP_Player.OnPlayerRespawn` _output_get (delegate `OnPlayerRespawn`))
  (`self.SetupKillCapsule`)
  (bind _asbp_arrow (cast `/Game/T5_PuzzleGame/Placeables/Interactables/BP_Arrow` (`ChildActorComponent.ChildActor` (`self.ChildActor`))))
  (set `self.Arrow1` _asbp_arrow)
  (add `ClickInteractComponent.OnActivateHighlight` (`self.ClickInteract`) (delegate `OnActivateHighlight_Event_0`))
  (`parent.ReceiveBeginPlay`)
  (add `GravitySwapComponent.OnFlipGravity` (`self.GravitySwap`) (delegate `CustomEvent_0`))
  (set `self.NormalLocation` (`SceneComponent.K2_GetComponentLocation` (`self.StaticMesh`)))
  (set `self.FlipLocation` (`SceneComponent.K2_GetComponentLocation` (`self.EndPos`)))
  (if (`GravitySwapComponent.bFlipGravity` (`self.GravitySwap`))
    (`SceneComponent.K2_SetWorldLocation` (`self.StaticMesh`) (`self.FlipLocation`) false false)))

(event `CustomEvent_0`
  (params (bInverted :type Boolean))
  (set `self.FlipGravity` bInverted)
  (set `self.MoveBox` true)
  (set `self.BoxMoveAlpha` 0.0)
  (set `self.LocationCache` (`SceneComponent.K2_GetComponentLocation` (`self.StaticMesh`))))

(event `self.ReceiveTick`
  (params (DeltaSeconds :type "Float (single-precision)"))
  (if (`self.MoveBox`)
    (set `self.BoxMoveAlpha` (+ (`self.BoxMoveAlpha`) (* DeltaSeconds 3.0)))
    (`SceneComponent.K2_SetWorldLocation` (`self.StaticMesh`) (`KismetMathLibrary.VLerp` (`self.LocationCache`) (select `bool` (`self.FlipGravity`) :`false` (`self.NormalLocation`) :`true` (`self.FlipLocation`)) (`KismetMathLibrary.FClamp` (`self.BoxMoveAlpha`))) true false)
    (if (`self.FlipGravity`)
      (if (== (`SceneComponent.K2_GetComponentLocation` (`self.StaticMesh`)) (`self.FlipLocation`) :`ErrorTolerance` 10.0)
        (set `self.MoveBox` false)
        (`GameplayStatics.PlaySound2D` "/Game/T5_PuzzleGame/Audio/CUE_ChandilerImpact_Cue.CUE_ChandilerImpact_Cue" 1.0 1.0 0.0 null null))
      (elif (== (`SceneComponent.K2_GetComponentLocation` (`self.StaticMesh`)) (`self.NormalLocation`) :`ErrorTolerance` 10.0)
        (set `self.MoveBox` false)
        (`GameplayStatics.PlaySound2D` "/Game/T5_PuzzleGame/Audio/CUE_ChandilerImpact_Cue.CUE_ChandilerImpact_Cue" 1.0 1.0 0.0 null null)))))

(event `OnPlayerRespawn`
  ;[1 1 1] OnPlayerRespawn
  (`SceneComponent.K2_SetWorldLocation` (`self.StaticMesh`) (select `bool` (`self.SavedFlipGravity`) :`false` (`self.NormalLocation`) :`true` (`self.FlipLocation`)) false true)
  (set `GravitySwapComponent.bFlipGravity` (`self.SavedFlipGravity`) (`self.GravitySwap`)))

(event `self.StopBox.OnBeginCursorOver`
  (params (TouchedComponent :type "PrimitiveComponent Object Reference"))
  ;[1 1 1] OnPlayerRespawn
  ;;[1 1 1] Display FlipGravity on cursor over(debugging)
  (`KismetSystemLibrary.PrintString` (`KismetStringLibrary.Concat_StrStr` "FlipGravity: " (`KismetStringLibrary.Conv_BoolToString` (`GravitySwapComponent.bFlipGravity` (`self.GravitySwap`))) " / SavedFlipGravity : " (`KismetStringLibrary.Conv_BoolToString` (`self.SavedFlipGravity`)))))

(event `self.ClickBox.OnComponentHit`
  (params (HitComponent :type "PrimitiveComponent Object Reference") (OtherActor :type "Actor Object Reference") (OtherComp :type "PrimitiveComponent Object Reference") (NormalImpulse :type "Vector Structure") (Hit :type "HitResult Structure (by ref)"))
  (if (== (`GameplayStatics.GetObjectClass` OtherActor) "/Game/T5_PuzzleGame/Core/BP_GravitySwappablePushBoxBase.BP_GravitySwappablePushBoxBase_C")
    (`PrimitiveComponent.SetAllPhysicsLinearVelocity` (`self.GetComponentByClass` OtherActor "/Script/Engine.StaticMeshComponent") (0.0 0.0 0.0) false)))

(event `self.KillCapsule.OnComponentBeginOverlap`
  (params (OverlappedComponent :type "PrimitiveComponent Object Reference") (OtherActor :type "Actor Object Reference") (OtherComp :type "PrimitiveComponent Object Reference") (OtherBodyIndex :type Integer) (bFromSweep :type Boolean) (SweepResult :type "HitResult Structure (by ref)"))
  ;[1 1 1] Kill Player
  (if (== OtherActor (`self.PlayerRef_0`))
    (`KismetSystemLibrary.PrintString` "Ready to kill")
    (set `self.KillPlayerOnSwap` true)))

(event `self.KillCapsule.OnComponentEndOverlap`
  (params (OverlappedComponent :type "PrimitiveComponent Object Reference") (OtherActor :type "Actor Object Reference") (OtherComp :type "PrimitiveComponent Object Reference") (OtherBodyIndex :type Integer))
  ;[1 1 1] Kill Player
  (if (== OtherActor (`self.PlayerRef_0`))
    (`KismetSystemLibrary.PrintString` "Unready")
    (set `self.KillPlayerOnSwap` false)))

(event `self.GravitySwap.OnFlipGravity`
  (params (bInverted :type Boolean))
  ;[1 1 1] Kill Player
  (`KismetSystemLibrary.Delay` (`self.KillDelay`))
  (if (`self.KillPlayerOnSwap`)
    (`/Game/T5_PuzzleGame/Characters/BP_Player.Die` (`self.PlayerRef_0`))))

(fn `BecomeActive`
  (`PrimitiveComponent.SetSimulatePhysics` (`self.StaticMesh`) false)
  (return))

(fn `IsFallingOntoPlayer`
  (params (Player :type "GravityCharacter Object Reference"))
  (returns (Value :type Boolean))
  (return false))

(fn `SetupKillCapsule`
  (locals (Distance :type "Float (double-precision)" :default 0.0))
  (if (`self.InnerLocation`)
    (`SceneComponent.K2_SetWorldLocation` (`self.KillCapsule`) (+ (- (`SceneComponent.K2_GetComponentLocation` (`self.StaticMesh`)) (`SceneComponent.K2_GetComponentLocation` (`self.EndPos`))) (/ (+ (`SceneComponent.K2_GetComponentLocation` (`self.StaticMesh`)) (`SceneComponent.K2_GetComponentLocation` (`self.EndPos`))) 2)) false false)
    (else
      (`SceneComponent.K2_SetWorldLocation` (`self.KillCapsule`) (/ (+ (`SceneComponent.K2_GetComponentLocation` (`self.StaticMesh`)) (`SceneComponent.K2_GetComponentLocation` (`self.EndPos`))) 2) false false)))
  (set `local.Distance` (`KismetMathLibrary.Vector_Distance` (`SceneComponent.K2_GetComponentLocation` (`self.StaticMesh`)) (`SceneComponent.K2_GetComponentLocation` (`self.EndPos`))))
  (if (>= (`CapsuleComponent.CapsuleRadius` (`self.KillCapsule`)) (/ (`local.Distance`) 4.0))
    (`CapsuleComponent.SetCapsuleRadius` (`self.KillCapsule`) (/ (`local.Distance`) 4.0) true))
  (`CapsuleComponent.SetCapsuleHalfHeight` (`self.KillCapsule`) (* (/ (`local.Distance`) 4.0) 0.9) true)
  (return))

(fn `UserConstructionScript`
  (`parent.UserConstructionScript`))