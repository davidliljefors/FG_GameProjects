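; BP_Road is a spline-driven road actor that builds its geometry in the construction script.
; It divides the spline into sections whose length is a fixed base length scaled by the actor's X scale, adding one spline mesh component per section.
; Each mesh takes local-space start and end positions and tangents from the spline, with tangent size capped at the section length.
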(fn `UserConstructionScript`
  (bind _returnvalue_x (`KismetMathLibrary.BreakVector` (`self.GetActorScale3D`)))
  (bind _spline (`self.Spline`))
  (bind _spline_2 (`self.Spline`))
  (set `self.SectionLenght` (* _returnvalue_x 345.0))
  (for _index (range (+ (`KismetMathLibrary.FTrunc` (/ (`SplineComponent.GetSplineLength` (`self.Spline`)) (`self.SectionLenght`))) 1))
    (bind _returnvalue (`AddComponent|NODE_AddSplineMeshComponent-0`))
    (bind _returnvalue_2 (* _index (`self.SectionLenght`)))
    (bind _returnvalue_3 (* (+ _index 1) (`self.SectionLenght`)))
    (`SplineMeshComponent.SetStartAndEnd` _returnvalue (`SplineComponent.GetLocationAtDistanceAlongSpline` _spline_2 _returnvalue_2 "Local") (`KismetMathLibrary.ClampVectorSize` (`SplineComponent.GetTangentAtDistanceAlongSpline` _spline_2 _returnvalue_2 "Local") 0.0 (`self.SectionLenght`)) (`SplineComponent.GetLocationAtDistanceAlongSpline` _spline _returnvalue_3 "Local") (`KismetMathLibrary.ClampVectorSize` (`SplineComponent.GetTangentAtDistanceAlongSpline` _spline _returnvalue_3 "Local") 0.0 (`self.SectionLenght`)) true)))