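; BP_SmartFence is an environment actor that builds a fence along an editable spline.
; Its construction script divides the spline length by SectionLenght and adds a spline mesh component per section, placed between local-space points at successive distances.
; Only start and end positions are set, as the clamped tangent calculations are left unused.
; Scale-based section length logic never runs, and the event graph is empty.
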(fn `UserConstructionScript`
  (for _index (range (+ (`KismetMathLibrary.FTrunc` (/ (`SplineComponent.GetSplineLength` (`self.Spline`)) (`self.SectionLenght`))) 1))
    (bind _returnvalue (`AddComponent|NODE_AddSplineMeshComponent-0`))
    (`SplineMeshComponent.SetStartAndEnd` _returnvalue (`SplineComponent.GetLocationAtDistanceAlongSpline` (`self.Spline`) (* _index (`self.SectionLenght`)) "Local") (0.0 0.0 0.0) (`SplineComponent.GetLocationAtDistanceAlongSpline` (`self.Spline`) (* (+ _index 1) (`self.SectionLenght`)) "Local") (0.0 0.0 0.0) true)))