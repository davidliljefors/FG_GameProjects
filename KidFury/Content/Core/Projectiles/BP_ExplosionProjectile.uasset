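; Exploding projectile that swells and changes color over its lifespan, then bursts into a ring of smaller BP_Projectile fragments.
; A timeline drives collision component scale and a dynamic material parameter, destroying the actor when finished.
; Timeline completion and hits both spawn ten evenly yawed fragments that inherit the instigator, if CanExplode is set.
; Overlapping a BP_ReinBat clears CanExplode, while any other overlap sets it.
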(event `self.ReceiveBeginPlay`
  (bind _staticmeshcomponent (`self.StaticMeshComponent`))
  (bind _instigator (`self.Instigator`))
  (bind (_spawntransfrom_location _spawntransfrom_rotation _spawntransfrom_scale) (`KismetMathLibrary.BreakTransform` (`self.SpawnTransfrom`)))
  (bind (_returnvalue_x _returnvalue_y _returnvalue_z) (`KismetMathLibrary.BreakVector` (`KismetMathLibrary.Conv_RotatorToVector` _spawntransfrom_rotation)))
  (bind (_returnvalue_location _returnvalue_rotation) (`KismetMathLibrary.BreakTransform` (`self.GetTransform` self)))
  (`parent.ReceiveBeginPlay`)
  (bind _returnvalue (`PrimitiveComponent.CreateDynamicMaterialInstance` _staticmeshcomponent 0 (`PrimitiveComponent.GetMaterial` _staticmeshcomponent 0) "None"))
  (set `self.Material` _returnvalue)
  (bind (_direction _scale _colorfade) (`Timeline|GrowBallOverTime` :`NewTime` (`self.GetLifeSpan`) :!via `PlayFromStart`)
    (:`Update`
      (`MaterialInstanceDynamic.SetScalarParameterValue` (`self.Material`) "ChangeColor" _colorfade)
      (`SceneComponent.SetWorldScale3D` (`self.CollisionComponent`) (`KismetMathLibrary.MakeVector` _scale _scale _scale)))
    (:`Finished`
      (set `self.SpawnTransfrom` (`KismetMathLibrary.MakeTransform` _returnvalue_location _returnvalue_rotation))
      (`self.K2_DestroyActor`)
      (if (`self.bCanExplode`)
        (for _index (range 10)
          (bind _returnvalue_2 (`|SpawnActorFromClass` "/Game/Core/Projectiles/BP_Projectile.BP_Projectile_C" (`KismetMathLibrary.MakeTransform` _spawntransfrom_location (`KismetMathLibrary.MakeRotator` _returnvalue_x _returnvalue_y (+ (* _index 36.0) _returnvalue_z)) _spawntransfrom_scale) "Undefined" "OverrideRootScale" _instigator (`self.FragmentBallsVelocity`) _instigator))
          (set `Projectile.ProjectileInstigator` (`self.ProjectileInstigator`) _returnvalue_2))))))

(event `self.ReceiveActorBeginOverlap`
  (params (OtherActor :type "Actor Object Reference"))
  (cast `/Game/Core/Characters/Player/BP_ReinBat` OtherActor
    (:`then`
      (set `self.bCanExplode` false))
    (:`CastFailed`
      (set `self.bCanExplode` true)))
  (`parent.ReceiveActorBeginOverlap` OtherActor))

(event `self.ReceiveTick`
  (params (DeltaSeconds :type "Float (single-precision)"))
  (`parent.ReceiveTick` DeltaSeconds))

(event `self.ReceiveHit`
  (params (MyComp :type "PrimitiveComponent Object Reference") (Other :type "Actor Object Reference") (OtherComp :type "PrimitiveComponent Object Reference") (bSelfMoved :type Boolean) (HitLocation :type "Vector Structure") (HitNormal :type "Vector Structure") (NormalImpulse :type "Vector Structure") (Hit :type "HitResult Structure (by ref)"))
  (bind (_spawntransfrom_location _spawntransfrom_rotation _spawntransfrom_scale) (`KismetMathLibrary.BreakTransform` (`self.SpawnTransfrom`)))
  (bind _instigator (`self.Instigator`))
  (bind (_returnvalue_location _returnvalue_rotation) (`KismetMathLibrary.BreakTransform` (`self.GetTransform` self)))
  (bind (_returnvalue_x _returnvalue_y _returnvalue_z) (`KismetMathLibrary.BreakVector` (`KismetMathLibrary.Conv_RotatorToVector` _spawntransfrom_rotation)))
  (if (or (!= Other "/Game/Core/Characters/DavidEnemy/BP_EnemyBase.BP_EnemyBase") (!= Other "/Game/Core/Projectiles/BP_Projectile.BP_Projectile"))
    (set `self.SpawnTransfrom` (`KismetMathLibrary.MakeTransform` _returnvalue_location _returnvalue_rotation))
    (if (`self.bCanExplode`)
      (for _index (range 10)
        (bind _returnvalue (`|SpawnActorFromClass` "/Game/Core/Projectiles/BP_Projectile.BP_Projectile_C" (`KismetMathLibrary.MakeTransform` _spawntransfrom_location (`KismetMathLibrary.MakeRotator` _returnvalue_x _returnvalue_y (+ (* _index 36.0) _returnvalue_z)) _spawntransfrom_scale) "Undefined" "OverrideRootScale" _instigator (`self.FragmentBallsVelocity`) _instigator))
        (set `Projectile.ProjectileInstigator` (`self.ProjectileInstigator`) _returnvalue)
        (`self.K2_DestroyActor`)))))

(fn `UserConstructionScript`
  (`parent.UserConstructionScript`))