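; Projectile that flies along a repeating spline-shaped path, named as a sinus wave, starting from its owner's location.
; On BeginPlay it caches its rotation and the owner's location, then a timeline samples the local-space SinusSpline by distance.
; Each sample is rotated by the cached rotation and offset from the start point, moving the actor without sweep.
; When the timeline finishes, the current location becomes the new start and the pattern replays.
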(event `self.ReceiveBeginPlay`
  (bind _sinusspline (`self.SinusSpline`))
  (`parent.ReceiveBeginPlay`)
  (set `self.Rotation` (`self.K2_GetActorRotation`))
  (set `self.StartLocation` (`self.K2_GetActorLocation` (`self.GetOwner`)))
  (bind (_direction _alpha) (`Timeline|SinusTimeLine` :`NewTime` (`self.InitialLifeSpan`) :!via `PlayFromStart` :!label _label)
    (:`Update`
      (set `self.Alpha` _alpha)
      (`self.K2_SetActorLocation` (+ (`self.StartLocation`) (`KismetMathLibrary.GreaterGreater_VectorRotator` (`SplineComponent.GetLocationAtDistanceAlongSpline` _sinusspline (`KismetMathLibrary.Lerp` 0.0 (`SplineComponent.GetSplineLength` _sinusspline) (`self.Alpha`)) "Local") (`self.Rotation`)))))
    (:`Finished`
      (set `self.StartLocation` (`self.K2_GetActorLocation`))
      (goto _label :!via `PlayFromStart`))))

(fn `UserConstructionScript`
  (`parent.UserConstructionScript`))