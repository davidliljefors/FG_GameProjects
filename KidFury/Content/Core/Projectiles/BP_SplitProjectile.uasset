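; BP_SplitProjectile is a projectile that fans out into a symmetric spread when it spawns.
; On BeginPlay, a root instance spawns pairs of copies of its own class, yawed left and right in multiples of DegreeOffset.
; Copies inherit the owner, instigators and velocity, and spawn with IsRoot false so the split does not recurse.
; Everything else is left to the parent class.
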(event `self.ReceiveBeginPlay`
  (bind _returnvalue (`self.GetTransform`))
  (bind _returnvalue_2 (`self.GetTransform`))
  (`parent.ReceiveBeginPlay`)
  (if (`self.bIsRoot`)
    (for _index (range 1 (+ (`self.ProjectilePairs`) 1))
      (bind _returnvalue_3 (`|SpawnActorFromClass` "BP_SplitProjectile_C" (`KismetMathLibrary.MakeTransform` (.location _returnvalue) (`KismetMathLibrary.MakeRotator` (.roll (.rotation _returnvalue)) (.pitch (.rotation _returnvalue)) (+ (.yaw (.rotation _returnvalue)) (* _index (`self.DegreeOffset`)))) (.scale _returnvalue)) "Undefined" "OverrideRootScale" (`self.GetOwner`) false (`self.Velocity`) (`self.Instigator`)))
      (set `Projectile.ProjectileInstigator` (`self.ProjectileInstigator`) _returnvalue_3)
      (bind _returnvalue_4 (`|SpawnActorFromClass` "BP_SplitProjectile_C" (`KismetMathLibrary.MakeTransform` (.location _returnvalue_2) (`KismetMathLibrary.MakeRotator` (.roll (.rotation _returnvalue_2)) (.pitch (.rotation _returnvalue_2)) (+ (.yaw (.rotation _returnvalue_2)) (* (* _index -1) (`self.DegreeOffset`)))) (.scale _returnvalue_2)) "Undefined" "OverrideRootScale" (`self.GetOwner`) false (`self.Velocity`) (`self.Instigator`)))
      (set `Projectile.ProjectileInstigator` (`self.ProjectileInstigator`) _returnvalue_4))))

(fn `UserConstructionScript`
  (`parent.UserConstructionScript`))