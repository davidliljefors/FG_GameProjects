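; BP_BurstProjectile is a projectile that, on BeginPlay, destroys itself and spawns a fan of projectiles from its collision component's location.
; A loop spawns BP_BurstProjectile, its own class, at stepped yaw offsets, passing the Instigator as owner and instigator.
; The spawn rotation uses forward-vector components as rotator angles rather than the component's actual rotation.
; Overlap and Tick events are disabled.
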(event `self.ReceiveBeginPlay`
  (bind _instigator (`self.Instigator`))
  (bind (_returnvalue_location _returnvalue_rotation _returnvalue_scale) (`KismetMathLibrary.BreakTransform` (`SceneComponent.K2_GetComponentToWorld` (`self.CollisionComponent`))))
  (bind (_returnvalue_x _returnvalue_y _returnvalue_z) (`KismetMathLibrary.BreakVector` (`KismetMathLibrary.Conv_RotatorToVector` _returnvalue_rotation)))
  (`parent.ReceiveBeginPlay`)
  (`self.K2_DestroyActor`)
  (for _index (range 4)
    (`|SpawnActorFromClass` "BP_BurstProjectile_C" (`KismetMathLibrary.MakeTransform` _returnvalue_location (`KismetMathLibrary.MakeRotator` _returnvalue_x _returnvalue_y (+ (* _index 36.0) _returnvalue_z)) _returnvalue_scale) "Undefined" "OverrideRootScale" _instigator 600.0 _instigator)))

(fn `UserConstructionScript`
  (`parent.UserConstructionScript`))