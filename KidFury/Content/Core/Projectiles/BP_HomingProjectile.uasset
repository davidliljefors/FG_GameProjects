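; Projectile that homes in on the first player character's current location.
; BeginPlay zeroes the projectile movement velocity, then Tick moves the actor toward the player with constant-speed interpolation at Speed, using a swept move.
; A ProjectileMovement homing setup in MoveToHomingTarget and a timeline velocity ramp remain in the graph but are disconnected, so neither runs.
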(event `self.ReceiveBeginPlay`
  (`parent.ReceiveBeginPlay`)
  (set `MovementComponent.Velocity` (0.0 0.0 0.0) (`self.ProjectileMovementComponent`)))

(event `self.ReceiveTick`
  (params (DeltaSeconds :type "Float (single-precision)"))
  (`self.K2_SetActorLocation` (`KismetMathLibrary.VInterpTo_Constant` (`self.K2_GetActorLocation`) (`self.K2_GetActorLocation` (`GameplayStatics.GetPlayerCharacter` 0)) DeltaSeconds (`self.Speed`)) true))

(fn `MoveToHomingTarget`
  (locals (ClosestDistance :type "Float (double-precision)" :default 999999.0))
  (bind _projectilemovementcomponent (`self.ProjectileMovementComponent`))
  (set `ProjectileMovementComponent.HomingTargetComponent` (`Actor.RootComponent` (`GameplayStatics.GetPlayerCharacter` 0)) _projectilemovementcomponent)
  (set `ProjectileMovementComponent.bIsHomingProjectile` true _projectilemovementcomponent)
  (set `MovementComponent.Velocity` (0.0 0.0 0.0) _projectilemovementcomponent)
  (set `ProjectileMovementComponent.HomingAccelerationMagnitude` (* (`self.Velocity`) 250.0) _projectilemovementcomponent))

(fn `UserConstructionScript`
  (`parent.UserConstructionScript`))