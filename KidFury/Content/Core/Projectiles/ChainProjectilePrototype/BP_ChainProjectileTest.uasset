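; Prototype chain projectile that spawns a second projectile and links the pair with a lightning beam that damages players.
; Each tick spins its mesh, moves the chain collision to the pair's midpoint, scales its Z by distance and updates the beam endpoints.
; Players overlapping the chain collision take fixed damage.
; When the second projectile becomes invalid, the collision and beam are destroyed once.
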(event `self.ReceiveBeginPlay`
  (bind _instigator (`self.Instigator`))
  (bind _returnvalue (`|SpawnActorFromClass` "/Game/Core/Projectiles/ChainProjectilePrototype/BP_ChainSecondProjectile.BP_ChainSecondProjectile_C" (`self.GetTransform`) "Undefined" "OverrideRootScale" _instigator (`self.ChainProjectileSpeed`) _instigator))
  (set `self.SecondChainProjectile` _returnvalue))

(event `self.ReceiveTick`
  (params (DeltaSeconds :type "Float (single-precision)"))
  (bind _p_chainlightning (`self.P_ChainLightning`))
  (bind _chaincollision (`self.ChainCollision`))
  (`SceneComponent.K2_AddLocalRotation` (`self.StaticMeshComponent`) (* (`KismetMathLibrary.MakeRotator` 0.0 -450.0) DeltaSeconds) false false)
  (`/Engine/EditorBlueprintResources/StandardMacros.IsValid` (`self.SecondChainProjectile`)
    (:`Is Valid`
      (bind _medianlocation (`self.GetMiddleOfVectors`))
      (`SceneComponent.K2_SetWorldLocation` _chaincollision _medianlocation false false)
      (bind _returndistance (`self.DistanceBetweenTwoVectors` (`SceneComponent.K2_GetComponentLocation` (`self.StaticMeshComponent`)) (`SceneComponent.K2_GetComponentLocation` (`self.ChainCollision`))))
      (`SceneComponent.SetWorldScale3D` _chaincollision (`KismetMathLibrary.MakeVector` 1.0 1.0 (* _returndistance 0.022)))
      (`ParticleSystemComponent.SetBeamSourcePoint` _p_chainlightning 0 (`SceneComponent.K2_GetComponentLocation` (`self.StaticMeshComponent`)) 0)
      (`ParticleSystemComponent.SetBeamTargetPoint` _p_chainlightning 0 (`SceneComponent.K2_GetComponentLocation` (`Projectile.StaticMeshComponent` (`self.SecondChainProjectile`))) 0))
    (:`Is Not Valid`
      (`/Engine/EditorBlueprintResources/StandardMacros.DoOnce` false
        (:`Completed`
          (`ActorComponent.K2_DestroyComponent` (`self.ChainCollision`))
          (`ActorComponent.K2_DestroyComponent` (`self.P_ChainLightning`)))))))

(event `self.ChainCollision.OnComponentBeginOverlap`
  (params (OverlappedComponent :type "PrimitiveComponent Object Reference") (OtherActor :type "Actor Object Reference") (OtherComp :type "PrimitiveComponent Object Reference") (OtherBodyIndex :type Integer) (bFromSweep :type Boolean) (SweepResult :type "HitResult Structure (by ref)"))
  (bind _asbp_player_character (cast `/Game/Core/Characters/Player/BP_PlayerCharacter` OtherActor))
  (`GameplayStatics.ApplyDamage` _asbp_player_character 25.0 null self))

(fn `DistanceBetweenTwoVectors`
  (params (VectorA :type "Vector Structure") (VectorB :type "Vector Structure"))
  (returns (ReturnDistance :type "Float (double-precision)"))
  (return (`KismetMathLibrary.Sqrt` (+ (`KismetMathLibrary.Square` (- (.x VectorA) (.x VectorB))) (`KismetMathLibrary.Square` (- (.y VectorA) (.y VectorB))) (`KismetMathLibrary.Square` (- (.z VectorA) (.z VectorB)))))))

(fn `GetMiddleOfVectors`
  (returns (MedianLocation :type "Vector Structure"))
  (bind _returnvalue (`self.K2_GetActorLocation`))
  (return (+ (/ (- (`self.K2_GetActorLocation` (`self.SecondChainProjectile`)) _returnvalue) 2.0) _returnvalue)))

(fn `GetNormalizedDistance`
  (returns (Distance :type "Float (double-precision)"))
  (return (+ (`KismetMathLibrary.NormalizeToRange` (`KismetMathLibrary.Vector_Distance` (`self.K2_GetActorLocation`) (`self.K2_GetActorLocation` (`self.SecondChainProjectile`))) 0.0 1000.0) 1.0)))

(fn `SetParticleSourceAndTarget`
  (bind _p_chainlightning (`self.P_ChainLightning`))
  (`ParticleSystemComponent.SetBeamSourcePoint` _p_chainlightning 0 (`SceneComponent.K2_GetComponentLocation` (`self.StaticMeshComponent`)) 0)
  (`ParticleSystemComponent.SetBeamTargetPoint` _p_chainlightning 0 (`SceneComponent.K2_GetComponentLocation` (`Projectile.StaticMeshComponent` (`self.SecondChainProjectile`))) 0))

(fn `UserConstructionScript`
  (`parent.UserConstructionScript`))