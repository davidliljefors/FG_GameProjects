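; BP_ExplosionBurstiburst is a short-lived projectile-burst actor that replaces itself with three BP_Projectile fragments on BeginPlay.
; It builds a spawn transform just ahead of its owner, destroys itself, then spawns the fragments with stepped yaw offsets and a shared fragment velocity, owned by the Instigator.
; Fragment rotations use the owner's forward-vector components directly as roll, pitch and yaw angles, so they do not follow its actual facing.
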(event `self.ReceiveBeginPlay`
  (bind _returnvalue (`self.GetOwner`))
  (bind (_spawntransfrom_location _spawntransfrom_rotation _spawntransfrom_scale) (`KismetMathLibrary.BreakTransform` (`self.SpawnTransfrom`)))
  (bind _instigator (`self.Instigator`))
  (bind (_returnvalue_location _returnvalue_rotation) (`KismetMathLibrary.BreakTransform` (`self.GetTransform` _returnvalue)))
  (bind (_returnvalue_x _returnvalue_y _returnvalue_z) (`KismetMathLibrary.BreakVector` (`KismetMathLibrary.Conv_RotatorToVector` _spawntransfrom_rotation)))
  (`parent.ReceiveBeginPlay`)
  (set `self.SpawnTransfrom` (`KismetMathLibrary.MakeTransform` (+ (`SceneComponent.GetForwardVector` (`Actor.RootComponent` _returnvalue)) _returnvalue_location) _returnvalue_rotation))
  (`self.K2_DestroyActor`)
  (for _index (range 1 4)
    (`|SpawnActorFromClass` "/Game/Core/Projectiles/BP_Projectile.BP_Projectile_C" (`KismetMathLibrary.MakeTransform` _spawntransfrom_location (`KismetMathLibrary.MakeRotator` _returnvalue_x _returnvalue_y (+ (* _index 10.0) _returnvalue_z)) _spawntransfrom_scale) "Undefined" "OverrideRootScale" _instigator (`self.FragmentBallsVelocity`) _instigator)))

(event `self.ReceiveActorBeginOverlap`
  (params (OtherActor :type "Actor Object Reference")))

(event `self.ReceiveTick`
  (params (DeltaSeconds :type "Float (single-precision)"))
  (`parent.ReceiveTick` DeltaSeconds))

(fn `UserConstructionScript`
  (`parent.UserConstructionScript`))