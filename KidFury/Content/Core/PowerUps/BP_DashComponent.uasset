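; Dash power-up component that moves a supplied actor quickly in a locked horizontal direction.
; The first DashEvent call locks direction from horizontal and vertical input on world axes, falling back to the actor's forward vector.
; Each call moves the actor one swept step scaled by speed, step size and delta time, until EndDashEvent releases the lock.
; An older dash sequence remains unconnected.
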(event `DashEvent`
  (params (Actor :type "Actor Object Reference") (MoveSpeed :type "Float (double-precision)") (StepSize :type "Float (double-precision)") (Horizontal :type "Float (double-precision)") (Vertical :type "Float (double-precision)"))
  (bind _returnvalue (`KismetMathLibrary.Vector_Normal2D` (+ (* (`KismetMathLibrary.Vector_Right`) Horizontal) (* (`KismetMathLibrary.Vector_Forward`) Vertical))))
  (if (not (`self.bIsDashing`))
    (if (> (`KismetMathLibrary.VSize` _returnvalue) 0.1)
      (set `self.DashDirection` _returnvalue)
      (else
        (set `self.DashDirection` (`Actor.GetActorForwardVector` Actor))))
    (set `self.bIsDashing` true))
  (`Actor.K2_SetActorLocation` Actor (+ (* (`self.DashDirection`) (* MoveSpeed StepSize (`GameplayStatics.GetWorldDeltaSeconds`))) (`Actor.K2_GetActorLocation` Actor)) true false))

(event `EndDashEvent`
  (set `self.bIsDashing` false))