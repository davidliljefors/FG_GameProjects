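; BP_HealthPickup is a pickup that heals the player when a GP2Character overlaps it, provided the player is alive and below max health.
; A one-shot branch adds percentage-based or flat health, clamped to max, briefly toggles the player's damage and healthbar-fade flags, then plays a sound and expires.
; It also clears the player's special-drop flag.
; At full health it plays an error sound and jitters its mesh through a timeline instead.
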(event `self.ReceiveActorBeginOverlap`
  (params (OtherActor :type "Actor Object Reference"))
  (bind _playermaxhealth (`self.PlayerMaxHealth`))
  (bind _asgp2character (cast `GP2Character` OtherActor))
  (if (`KismetSystemLibrary.IsValid` _asgp2character)
    (`self.GetVariables`)
    (if (not (`/Game/Core/Characters/Player/BP_PlayerCharacter.IsDead` (`self.PlayerCharacter`)))
      (if (< (`self.PlayerHealth`) (`self.PlayerMaxHealth`))
        (`/Engine/EditorBlueprintResources/StandardMacros.DoOnce` false
          (:`Completed`
            (set `/Game/Core/Characters/Player/BP_PlayerCharacter.IsHealthbarFaded` false (`self.PlayerCharacter`))
            (set `/Game/Core/Characters/Player/BP_PlayerCharacter.CanTakeDamage` true (`self.PlayerCharacter`))
            (if (`self.bUsePercentHealing`)
              (bind _output_get (set `/Game/Core/Characters/Player/BP_PlayerCharacter.Health` (+ (* _playermaxhealth (`self.AddPercentOfMaxhealth`)) (`self.PlayerHealth`)) (`self.PlayerCharacter`)))
              (if (> _output_get _playermaxhealth)
                (set `/Game/Core/Characters/Player/BP_PlayerCharacter.Health` (`self.PlayerMaxHealth`) (`self.PlayerCharacter`) :!label _label))
              (else
                (bind _output_get_2 (set `/Game/Core/Characters/Player/BP_PlayerCharacter.Health` (+ (`self.PlayerHealth`) (`self.AddHealthAmount`)) (`self.PlayerCharacter`)))
                (if (> _output_get_2 (`self.PlayerMaxHealth`))
                  (goto _label)
                  (else
                    _))))
            (`KismetSystemLibrary.Delay` 0.05)
            (`GameplayStatics.PlaySoundAtLocation` "/Game/Sounds/Cue_HealthPickup.Cue_HealthPickup" (`self.K2_GetActorLocation`) (struct) 1.0 1.0 0.0 null null null)
            (set `/Game/Core/Characters/Player/BP_PlayerCharacter.CanTakeDamage` false (`self.PlayerCharacter`))
            (set `/Game/Core/Characters/Player/BP_PlayerCharacter.IsHealthbarFaded` true (`self.PlayerCharacter`))
            (`self.SetLifeSpan` 0.05)
            (set `/Game/Core/Characters/Player/BP_PlayerCharacter.bSpecialHealthPickupDroped` false (`self.PlayerCharacter`))))
        (else
          (`GameplayStatics.PlaySound2D` "/Game/Sounds/Wrong_Cue.Wrong_Cue" 1.0 1.0 0.0 null null)
          ;[1 1 1] Jitter when player have full health
          (bind (_direction _lerp) (`Timeline|PickUpJitter` :!via `PlayFromStart`)
            (:`Update`
              (`SceneComponent.K2_SetRelativeLocation` (`self.StaticMeshComponent`) (`KismetMathLibrary.VLerp` (0.0 0.0 0.0) (30.0 30.0 0.0) _lerp) true false))))))))

(fn `GetVariables`
  (bind _asbp_player_character (cast `/Game/Core/Characters/Player/BP_PlayerCharacter` (`GameplayStatics.GetPlayerPawn` 0)))
  (bind _output_get (set `self.PlayerCharacter` _asbp_player_character))
  (set `self.PlayerHealth` (`/Game/Core/Characters/Player/BP_PlayerCharacter.Health` _output_get))
  (set `self.PlayerMaxHealth` (`/Game/Core/Characters/Player/BP_PlayerCharacter.MaxHealth` _output_get)))

(fn `UserConstructionScript`)