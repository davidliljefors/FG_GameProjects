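; Player's bat that charges swings and deflects incoming projectiles at enemies.
; A timeline ramps force and the charge sound filter, then triggers full-charge animation and audio through a gate that swinging closes.
; Swing briefly enables cap collision; overlapped projectiles are hidden and replaced by player projectiles aimed at the nearest enemy in front, or along player facing otherwise.
; Full charge spawns faster, larger fire projectiles.
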(event `self.ReceiveBeginPlay`
  (`PrimitiveComponent.SetCollisionEnabled` (`self.caps`) "NoCollision")
  (bind _returnvalue (`AddComponent|NODE_AddAudioComponent-0`))
  (bind _output_get (set `self.BurningSound` _returnvalue))
  (`AudioComponent.Stop` _output_get))

(event `ChargeSwing`
  (set `self.IsFullyCharged` false)
  (`|ExecutionSequence`
    (:`then_0`
      (`AudioComponent.FadeIn` (`self.ChargeSound`) 0.8 1.0 0.0 "Linear")
      (goto _label :!via `Open`))
    (:`then_1`
      (bind (_direction _forcemultiplier) (`Timeline|Timeline_1` :!via `PlayFromStart`)
        (:`Update`
          (bind _output_get (set `self.ForceMultiplier` _forcemultiplier))
          (`AudioComponent.SetLowPassFilterFrequency` (`self.ChargeSound`) (+ 50.0 (* _output_get 1000.0))))
        (:`Finished`
          (`self.StopChargeSound`)
          ;[1 1 1] Stopping charge effects from playing after swing
          (`/Engine/EditorBlueprintResources/StandardMacros.Gate` true :!label _label
            (:`Exit`
              (set `self.IsFullyCharged` true)
              (`AudioComponent.Play` (`self.MaxSwing`) 0.0)
              (bind _asabp_character (cast `/Game/3D/Animation/ABP_Character` (`SkeletalMeshComponent.GetAnimInstance` (`Character.Mesh` (`self.Player`)))))
              (`/Game/3D/Animation/ABP_Character.ChargeMax` _asabp_character)
              (`AudioComponent.FadeIn` (`self.MaxChargeSound`) 0.03 1.0 0.0 "Linear")
              (`AudioComponent.FadeIn` (`self.BurningSound`) 0.1 1.0 0.0 "Linear"))))))))

(event `PlaySwingSound`
  (bind _swingsound (`self.SwingSound`))
  (`AudioComponent.SetPitchMultiplier` _swingsound (+ (`KismetMathLibrary.RandomFloatInRange` 1.1 1.3) (* (`self.LastForce`) 0.2)))
  (`AudioComponent.Play` _swingsound 0.0))

(event `StopChargeSound`
  (`AudioComponent.FadeOut` (`self.ChargeSound`) 0.2 0.0 "Logarithmic"))

(event `Swing`
  (bind _burningsound (`self.BurningSound`))
  ;[1 0.75 0.3102] Swing, enable collision and disable after set time
  (`|ExecutionSequence`
    (:`then_0`
      ;[1 1 1] Close all gates
      (`|ExecutionSequence`
        (:`then_0`
          (goto _label :!via `Close`))))
    (:`then_1`
      (`/Game/Core/Characters/Player/BP_PlayerCharacter.SetSpeedForSeconds` (`self.Player`) 0.15 150.0)
      (set `self.LastForce` (`self.ForceMultiplier`))
      (`self.StopChargeSound`)
      (`PrimitiveComponent.SetCollisionEnabled` (`self.caps`) "QueryAndPhysics")
      (`self.PlaySwingSound`)
      (if (`AudioComponent.IsPlaying` _burningsound)
        (`AudioComponent.FadeOut` _burningsound 0.5 0.0 "Linear"))
      (`KismetSystemLibrary.RetriggerableDelay` (`self.SwingDuration`))
      (`PrimitiveComponent.SetCollisionEnabled` (`self.caps`) "NoCollision"))))

(event `self.caps.OnComponentBeginOverlap`
  (params (OverlappedComponent :type "PrimitiveComponent Object Reference") (OtherActor :type "Actor Object Reference") (OtherComp :type "PrimitiveComponent Object Reference") (OtherBodyIndex :type Integer) (bFromSweep :type Boolean) (SweepResult :type "HitResult Structure (by ref)"))
  (bind _baseprojectilespeed (`self.BaseProjectileSpeed`))
  ;[1 1 1] Ball hit, deflect it
  (if (`KismetMathLibrary.ClassIsChildOf` (`GameplayStatics.GetObjectClass` OtherActor) "/Script/GP2.Projectile")
    (`self.DestroyAndHide` OtherActor)
    (`self.OnBallDeflected`)
    (if (`self.IsFullyCharged`)
      (`self.DeflectToNearest` OtherActor (* _baseprojectilespeed 8.0) 0.0 2000.0 (3.0 1.0 1.0) "/Game/Core/Characters/Player/BP_PlayerFireProjectile.BP_PlayerFireProjectile_C")
      (else
        (`self.DeflectToNearest` OtherActor _baseprojectilespeed (* (- (`self.LastForce`) 1.0) (`self.MaxInaccuracy`)) 2000.0 (1.5 1.0 1.0) "/Game/Core/Characters/Player/BP_PlayerProjectile.BP_PlayerProjectile_C")))
    (`AudioComponent.Play` (`self.HitSound`) 0.0)))

(fn `DeflectProjectile`
  (params (Projectile :type "Actor Object Reference") (NewVelocity :type "Float (double-precision)") (`Inaccuracy (Deg)` :type "Float (double-precision)") (Class :type "/Game/Core/Characters/Player/BP_PlayerProjectile Class Reference"))
  (returns (DeflectedProjectile :type "/Game/Core/Characters/Player/BP_PlayerProjectile Object Reference"))
  (locals (ConstantVelocity :type "Float (double-precision)" :default 2000.0))
  (bind (_returnvalue_location _returnvalue_rotation) (`KismetMathLibrary.BreakTransform` (`self.GetTransform` (`self.Player`))))
  (`self.SetLifeSpan` Projectile 0.5)
  (`self.SetActorEnableCollision` Projectile false)
  (`self.SetActorHiddenInGame` Projectile true)
  (bind _outputpin (`self.SpawnProjectile` _returnvalue_location (`self.DoInaccarcy` _returnvalue_rotation (`local.Inaccuracy (Deg)`)) (`local.NewVelocity`) (`self.Player`) (1.0 1.0 1.0) Class))
  (return _outputpin))

(fn `DeflectToNearest`
  (params (Projectile :type "Actor Object Reference") (NewVelocity :type "Float (double-precision)") (`Inaccuracy (Deg)` :type "Float (double-precision)") (EnemyRadius :type "Float (double-precision)") (Transform :type "Vector Structure") (Class :type "/Game/Core/Characters/Player/BP_PlayerProjectile Class Reference"))
  (returns (DeflectedProjectile :type "/Game/Core/Characters/Player/BP_PlayerProjectile Object Reference"))
  (locals (ConstantVelocity :type "Float (double-precision)" :default 2000.0))
  (bind _returnvalue (`self.K2_GetActorLocation` (`local.Projectile`)))
  (bind _returnvalue_2 (`GP2Character.GetNearestEnemyInFront` (`self.Player`) EnemyRadius 0.3))
  (`/Engine/EditorBlueprintResources/StandardMacros.IsValid` _returnvalue_2
    (:`Is Valid`
      (bind _outputpin (`self.SpawnProjectile` _returnvalue (`self.DoInaccarcy` (`KismetMathLibrary.FindLookAtRotation` _returnvalue (`self.K2_GetActorLocation` _returnvalue_2)) (`local.Inaccuracy (Deg)`)) (`local.NewVelocity`) (`self.Player`) Transform Class))
      (return _outputpin))
    (:`Is Not Valid`
      (bind _deflectedprojectile (`self.DeflectProjectile` (`local.Projectile`) (`local.NewVelocity`) (`local.Inaccuracy (Deg)`) Class))
      (return _deflectedprojectile))))

(fn `SpawnProjectile`
  (params (SpawnTransform_Location :type "Vector Structure") (SpawnTransform_Rotation :type "Rotator Structure") (Velocity :type "Float (double-precision)") (Owner :type "Pawn Object Reference") (TransformScaleBall :type "Vector Structure" :default (1.0 1.0 1.0)) (Class :type "/Game/Core/Characters/Player/BP_PlayerProjectile Class Reference"))
  (returns (OutputPin :type "/Game/Core/Characters/Player/BP_PlayerProjectile Object Reference"))
  (bind _returnvalue (`|SpawnActorFromClass` Class (`KismetMathLibrary.MakeTransform` SpawnTransform_Location SpawnTransform_Rotation TransformScaleBall) "Undefined" "OverrideRootScale" Owner Velocity Owner))
  (`self.SetupProjectileCollision` _returnvalue)
  (set `Projectile.ProjectileInstigator` (`Pawn.GetController` Owner) _returnvalue)
  (return _returnvalue))

(fn `UserConstructionScript`)