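; Player controller that switches combat music, handles menu back navigation and offers marketing capture tools.
; BeginPlay caches the smooth camera, HUD and game mode, then creates two audio components that combat events crossfade between.
; Exit closes main or pause sub-windows, resumes or opens the pause menu; gamepad right face button shares this logic without opening pause.
; In marketing mode, F takes screenshots and M toggles a level sequence.
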(event `SetUpAudio`
  (bind _returnvalue (`AddComponent|NODE_AddAudioComponent-3`))
  (bind _output_get (set `self.CombatMusic` _returnvalue))
  (`AudioComponent.Stop` _output_get)
  (bind _returnvalue_2 (`AddComponent|NODE_AddAudioComponent-5`))
  (bind _output_get_2 (set `self.OutOfCombat` _returnvalue_2))
  (`AudioComponent.Stop` _output_get_2))

(event `StartMusic`
  (`AudioComponent.FadeIn` (`self.OutOfCombat`) 1.0 1.0 0.0 "Linear"))

(event `ExitCombat`
  (if (`AudioComponent.IsPlaying` (`self.CombatMusic`))
    (`AudioComponent.FadeOut` (`self.CombatMusic`) 1.0 0.0 "Linear"))
  (`AudioComponent.FadeIn` (`self.OutOfCombat`) 1.0 1.0 0.0 "Linear"))

(event `Key|F`
  (params (Key :type "Key Structure"))
  ;[0.0405 0.5729 0] Marketing tool
  (:`Released`
    (if (`self.MarketingModeEnabled`)
      (`/Game/Core/GameModes/BP_MainGameMode.TakeScreenShot` (`self.GameMode`) "NewEnumerator0"))))

(event `EnterCombat`
  (if (`AudioComponent.IsPlaying` (`self.OutOfCombat`))
    (`AudioComponent.FadeOut` (`self.OutOfCombat`) 1.0 0.0 "Linear"))
  (`AudioComponent.FadeIn` (`self.CombatMusic`) 1.0 1.0 0.0 "Linear"))

(event `Key|M`
  (params (Key :type "Key Structure"))
  (bind _marketingcutscene (`self.MarketingCutscene`))
  ;[0.0405 0.5729 0] Marketing tool
  (:`Released`
    (if (`self.MarketingModeEnabled`)
      (if (`MovieSceneSequencePlayer.IsPlaying` _marketingcutscene)
        (`MovieSceneSequencePlayer.Stop` _marketingcutscene)
        (else
          (`MovieSceneSequencePlayer.Play` _marketingcutscene))))))

(event `self.ReceiveBeginPlay`
  (bind _returnvalue (`GameplayStatics.GetActorOfClass` "/Game/Core/Camera/BP_SmoothCamera.BP_SmoothCamera_C"))
  (set `self.SmoothCamera` _returnvalue)
  (bind _ashud_gp2 (cast `/Game/UI/HUD_GP2` (`self.GetHUD`)))
  (set `self.HUD` _ashud_gp2)
  (`self.SetUpAudio`)
  (bind _asbp_main_game_mode (cast `/Game/Core/GameModes/BP_MainGameMode` (`GameplayStatics.GetGameMode`)))
  (set `self.GameMode` _asbp_main_game_mode)
  (bind (_outactor _returnvalue_2) (`LevelSequencePlayer.CreateLevelSequencePlayer` "/Game/Maps/CinematicActors/MarketingSequence.MarketingSequence"))
  (set `self.MarketingCutscene` _returnvalue_2))

(event `InputAction|Exit` :paused true
  (params (Key :type "Key Structure"))
  (bind _hud (`self.HUD`))
  (bind _pausemenu (`/Game/UI/HUD_GP2.PauseMenu` _hud))
  (bind _mainmenu (`/Game/UI/HUD_GP2.MainMenu` (`self.HUD`)))
  (bind _mainmenu_2 (`/Game/UI/HUD_GP2.MainMenu` (`self.HUD`)))
  (bind _pausemenu_2 (`/Game/UI/HUD_GP2.PauseMenu` _hud))
  ;[0.9912 0.3798 1] Exit (Pause Game) - Spaghetti Delux
  (:`Pressed`
    (if (`/Game/UI/HUD_GP2.IsMainMenuOpen` (`self.HUD`))
      (if (or (`Widget.IsInViewport` (`/Game/UI/Widget_MainMenu.OptionsMenu` _mainmenu_2)) (`Widget.IsInViewport` (`/Game/UI/Widget_MainMenu.Credits` _mainmenu_2)) (`Widget.IsInViewport` (`/Game/UI/Widget_MainMenu.Instructions` _mainmenu_2))) :!label _label
        (`/Game/UI/Widget_MainMenu.CloseWindow` _mainmenu)
        (if (`Widget.IsInViewport` _mainmenu)
          (`/Game/UI/Widget_MainMenu.OpenEventTick` _mainmenu)
          (else
            (`/Game/UI/HUD_GP2.OpenWidget` (`self.HUD`) "NewEnumerator1"))))
      (elif (`/Game/UI/HUD_GP2.IsPauseMenuOpen` (`self.HUD`))
        (if (`/Game/UI/Widget_MainMenu.HasChildWidgets` _pausemenu_2) :!label _label_2
          (`/Game/UI/Widget_MainMenu.CloseWindow` _pausemenu :!label _label_3)
          (if (`Widget.IsInViewport` _pausemenu)
            (`/Game/UI/Widget_MainMenu.OpenEventTick` _pausemenu)
            (else
              (`/Game/UI/HUD_GP2.OpenWidget` (`self.HUD`) "NewEnumerator4")))
          (else
            (`/Game/UI/Widget_MainMenu.FadeOutAudio` _pausemenu_2)
            (`/Game/UI/HUD_GP2.CloseWidget` (`self.HUD`) "NewEnumerator4")
            (`/Game/UI/HUD_GP2.OpenWidget` (`self.HUD`) "NewEnumerator3")
            (`GameplayStatics.SetGamePaused` false)))
        (elif (`/Game/UI/Widget_MainMenu.HasChildWidgets` _pausemenu)
          (goto _label_3)
          (else
            (`/Game/UI/HUD_GP2.CloseWidget` (`self.HUD`) "NewEnumerator3")
            (`/Game/UI/HUD_GP2.OpenWidget` (`self.HUD`) "NewEnumerator4")))))))

(event `Key|Gamepad_FaceButton_Right` :paused true
  (params (Key :type "Key Structure"))
  (bind _hud (`self.HUD`))
  ;[0.9912 0.3798 1] Exit (Pause Game) - Spaghetti Delux
  (:`Pressed`
    (if (`/Game/UI/HUD_GP2.IsMainMenuOpen` (`self.HUD`))
      (goto _label)
      (elif (`/Game/UI/HUD_GP2.IsPauseMenuOpen` _hud)
        (goto _label_2)
        (elif (`/Game/UI/Widget_MainMenu.HasChildWidgets` (`/Game/UI/HUD_GP2.PauseMenu` _hud))
          (goto _label_3))))))

(fn `UserConstructionScript`)