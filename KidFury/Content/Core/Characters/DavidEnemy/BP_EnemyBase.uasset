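; Base enemy character that faces its AI Blackboard target, takes damage from the player and dies in an explosion of parts.
; ActivateEnemy enables tick and binds damage handling, where hits flash dynamic materials, update the health bar and set the attacker as target.
; Death launches parts along the projectile's direction and rolls a health pickup, optionally boosted once by the player's missing health.
; Overlapping a BP_ReinBat pushes its player back with force-field effects.
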(event `self.ReceiveTick`
  (params (DeltaSeconds :type "Float (single-precision)"))
  (bind _asactor (cast `Actor` (`BlackboardComponent.GetValueAsObject` (`AIController.Blackboard` (`AIBlueprintHelperLibrary.GetAIController` self)) "TargetActor")))
  (bind (_returnvalue_roll _returnvalue_pitch _returnvalue_yaw) (`KismetMathLibrary.BreakRotator` (`KismetMathLibrary.FindLookAtRotation` (`self.K2_GetActorLocation`) (`self.K2_GetActorLocation` _asactor))))
  (`SceneComponent.K2_SetWorldRotation` (`self.Mesh`) (`KismetMathLibrary.MakeRotator` _returnvalue_roll _returnvalue_pitch (+ _returnvalue_yaw -90.0)) false false))

(event `ActivateEnemy`
  (`SceneComponent.SetVisibility` (`self.CapsuleComponent`) true true)
  (`self.SetActorTickEnabled` true)
  (add `self.OnTakeAnyDamage` (delegate `OnTakeAnyDamage_Event_0`))
  (add `self.OnEnemyAttack` (delegate `EnemyAttacking`)))

(event `EnemyAttacking`
  (`GameplayStatics.PlaySoundAtLocation` "/Game/Sounds/Enemy/Cue_EnemyThrowSound.Cue_EnemyThrowSound" (`self.K2_GetActorLocation`) (struct) 1.0 1.0 0.0 null null null))

(event `OnTakeAnyDamage_Event_0` :!signature `self.OnTakeAnyDamage`
  (params (DamagedActor :type "Actor Object Reference") (Damage :type "Float (double-precision)") (DamageType :type "DamageType Object Reference") (InstigatedBy :type "Controller Object Reference") (DamageCauser :type "Actor Object Reference"))
  (bind _blackboard (`AIController.Blackboard` (`AIBlueprintHelperLibrary.GetAIController` self)))
  (if (`KismetMathLibrary.ClassIsChildOf` (`GameplayStatics.GetObjectClass` InstigatedBy) "/Script/GP2.GP2PlayerController")
    (`|ExecutionSequence`
      (:`then_0`
        (`self.Blink` (struct :`R` 1.0 :`A` 1.0)))
      (:`then_1`
        (`GameplayStatics.PlaySoundAtLocation` "/Game/Sounds/Enemy/Cue_EnemyDamage.Cue_EnemyDamage" (`self.K2_GetActorLocation` DamagedActor) (struct) 1.0 1.0 0.0 null null null)
        (`self.Decrease Health` Damage)
        (if (> (`self.Health`) 0.0)
          (`BlackboardComponent.SetValueAsObject` _blackboard "TargetActor" (`Controller.K2_GetPawn` InstigatedBy))
          (`BlackboardComponent.SetValueAsBool` _blackboard "bHasTarget" true)
          (`ActorComponent.SetActive` (`self.P_EnemyHit2`) true true)
          (`self.SetLifeSpan` DamageCauser 0.01)
          (else
            (`/Engine/EditorBlueprintResources/StandardMacros.DoOnce` false
              (:`Completed`
                (`self.Die` DamageCauser)))))))))

(event `Blink`
  (params (Value :type "LinearColor Structure"))
  (bind (_direction _damagedfade) (`Timeline|DamageBlink` :!via `PlayFromStart`)
    (:`Update`
      (for _array_element (`self.Materials`)
        (`MaterialInstanceDynamic.SetVectorParameterValue` _array_element "DamagedColor" Value)
        (`MaterialInstanceDynamic.SetScalarParameterValue` _array_element "DamagedFade" _damagedfade)))))

(event `CustomEvent_0` :!signature `self.OnDeath`
  (params (KilledEnemy :type "/Game/Core/Characters/DavidEnemy/BP_EnemyBase Object Reference"))
  ;[1 1 1] spawn emitters on death
  (for _ (range 11)
    (`GameplayStatics.SpawnEmitterAtLocation` "/Game/SeanTest/Vfx/P_EnemyHit_01.P_EnemyHit_01" (`KismetMathLibrary.RandomPointInBoundingBox` (`self.K2_GetActorLocation`) (75.0 75.0 25.0)))))

(event `self.CapsuleComponent.OnComponentHit`
  (params (HitComponent :type "PrimitiveComponent Object Reference") (OtherActor :type "Actor Object Reference") (OtherComp :type "PrimitiveComponent Object Reference") (NormalImpulse :type "Vector Structure") (Hit :type "HitResult Structure (by ref)"))
  (bind (_bblockinghit _binitialoverlap _time _distance _location _impactpoint _normal) (`GameplayStatics.BreakHitResult` Hit))
  (if (`KismetMathLibrary.ClassIsChildOf` (`GameplayStatics.GetObjectClass` OtherActor) "/Game/Core/Characters/Player/BP_PlayerProjectile.BP_PlayerProjectile_C")
    (`GameplayStatics.SpawnEmitterAtLocation` "/Game/SeanTest/Vfx/P_EnemyHit_01.P_EnemyHit_01" (+ _location (* _normal 50)))))

(event `SetArmorMaterials`
  (params (StaticMeshes :type "Array of StaticMeshComponent Object Reference"))
  (for _array_element StaticMeshes
    (for (_array_element_2 _array_index) (`MeshComponent.GetMaterials` _array_element)
      (bind _returnvalue (`PrimitiveComponent.CreateDynamicMaterialInstance` _array_element _array_index _array_element_2 "None"))
      (`KismetArrayLibrary.Array_Add` (`self.Materials`) _returnvalue))))

(event `self.CapsuleComponent.OnComponentBeginOverlap`
  (params (OverlappedComponent :type "PrimitiveComponent Object Reference") (OtherActor :type "Actor Object Reference") (OtherComp :type "PrimitiveComponent Object Reference") (OtherBodyIndex :type Integer) (bFromSweep :type Boolean) (SweepResult :type "HitResult Structure (by ref)"))
  (bind _returnvalue (`self.K2_GetActorLocation`))
  (bind _asbp_rein_bat (cast `/Game/Core/Characters/Player/BP_ReinBat` OtherActor))
  (`self.Blink` (struct :`R` 1.0 :`G` 1.0 :`B` 1.0 :`A` 1.0))
  (`/Game/Core/Characters/Player/BP_PlayerCharacter.PushBack` (`/Game/Core/Characters/Player/BP_ReinBat.Player` _asbp_rein_bat) _returnvalue (`self.PushForce`))
  (if true
    (`ActorComponent.SetActive` (`self.P_PushForce`) true true)
    (`GameplayStatics.PlayWorldCameraShake` "/Game/Core/Camera/BP_CameraShake.BP_CameraShake_C" (`self.K2_GetActorLocation` (`GameplayStatics.GetPlayerCharacter` 0)) 0.0 5000.0 0.5)
    (`GameplayStatics.PlaySoundAtLocation` "/Game/Sounds/Enemy/Cue_ForceField.Cue_ForceField" _returnvalue (struct) 1.0 1.0 0.0 null null null)))

(fn `CheckDeath`
  (if (<= (`self.Health`) 0.0)
    (set `self.bIsAlive` false)))

(fn `Decrease Health`
  (params (Amount :type "Float (double-precision)"))
  (if (`self.bIsAlive`)
    (bind _output_get (set `self.Health` (- (`self.Health`) Amount)))
    (bind _aswbp_enemy_health_bar (cast `/Game/UI/WBP_EnemyHealthBar` (`WidgetComponent.GetUserWidgetObject` (`self.Healthbar`))))
    (`/Game/UI/WBP_EnemyHealthBar.SetFIll` _aswbp_enemy_health_bar (/ _output_get (`self.MaxHealth`)))
    (return)
    (else
      (return))))

(fn `Die`
  (params (DamageCauser :type "Actor Object Reference"))
  (set `self.bIsAlive` false)
  (set `self.Health` 0.0)
  (`PrimitiveComponent.SetCollisionEnabled` (`self.CapsuleComponent`) "NoCollision")
  (`self.Explode on Death` 700.0 (`local.DamageCauser`))
  (`self.SpawnHealthPickup`)
  (`GameplayStatics.PlaySoundAtLocation` "/Game/Sounds/Enemy/Cue_EnemyDeath.Cue_EnemyDeath" (`CharacterMovementComponent.GetLastUpdateLocation` (`self.CharacterMovement`)) (struct) 1.0 1.0 0.0 null null null)
  (`self.OnDeath` self)
  (`self.SetLifeSpan` 0.01))

(fn `Explode on Death`
  (params (Force :type "Float (double-precision)" :default 1000.0) (DamageCauser :type "Actor Object Reference"))
  (bind (_returnvalue_location _returnvalue_rotation) (`KismetMathLibrary.BreakTransform` (`SceneComponent.K2_GetComponentToWorld` (`self.CapsuleComponent`))))
  (`GameplayStatics.SpawnEmitterAtLocation` "/Game/SeanTest/Vfx/P_Explosion_01.P_Explosion_01" (`self.K2_GetActorLocation`))
  (bind _asprojectile (cast `Projectile` (`local.DamageCauser`)))
  (for _array_element (`.PropsToSpawn_5_429783134EA15D30597662A21E9279FF` (break `/Game/Core/Characters/DavidEnemy/ExplodeProps/FExplodeProps` (`self.ExplodeParts`)))
    (`|SpawnActorFromClass` _array_element (`KismetMathLibrary.MakeTransform` _returnvalue_location _returnvalue_rotation (`SceneComponent.K2_GetComponentScale` (`self.Mesh`))) "Undefined" "OverrideRootScale" null (`local.Force`) 60.0 (`KismetMathLibrary.Normal` (`MovementComponent.Velocity` (`Projectile.ProjectileMovementComponent` _asprojectile))) null)))

(fn `SetInitialVariables`)

(fn `SpawnHealthPickup`
  (bind _returnvalue (`KismetMathLibrary.RandomFloatInRange` 0.0 1.0))
  (if (`self.bIncludePlayerHealthInDropChance`)
    (bind _asbp_player_character (cast `/Game/Core/Characters/Player/BP_PlayerCharacter` (`GameplayStatics.GetPlayerCharacter` 0)))
    (if (`/Game/Core/Characters/Player/BP_PlayerCharacter.bSpecialHealthPickupDroped` _asbp_player_character)
      (if (or (<= _returnvalue (`self.PercentToDropHealthPickup`)) (> _returnvalue 1.0)) :!label _label
        (`|SpawnActorFromClass` "/Game/Core/Pickups/BP_HealthPickup.BP_HealthPickup_C" (`self.GetTransform` self) "Undefined" "OverrideRootScale" null null :!label _label_2)
        (`GameplayStatics.PlaySoundAtLocation` "/Game/Sounds/Cue_HealthPickup.Cue_HealthPickup" (`self.K2_GetActorLocation`) (struct) 1.0 1.0 0.0 null null null))
      (else
        (bind _returnvalue_2 (/ (- 1.0 (`KismetMathLibrary.NormalizeToRange` (`/Game/Core/Characters/Player/BP_PlayerCharacter.Health` _asbp_player_character) 0.0 (`/Game/Core/Characters/Player/BP_PlayerCharacter.MaxHealth` _asbp_player_character))) 3.0))
        (if (> _returnvalue_2 0.0)
          (bind _returnvalue_3 (+ (`self.PercentToDropHealthPickup`) _returnvalue_2))
          (if (or (<= (`KismetMathLibrary.RandomFloatInRange` 0.0 1.0) _returnvalue_3) (> _returnvalue_3 1.0))
            (set `/Game/Core/Characters/Player/BP_PlayerCharacter.bSpecialHealthPickupDroped` true _asbp_player_character)
            (goto _label_2))
          (else
            (goto _label)))))
    (else
      (goto _label))))

(fn `UserConstructionScript`
  (bind _mesh (`self.Mesh`))
  (bind _legs (`self.Legs`))
  (for (_array_element _array_index) (`MeshComponent.GetMaterials` _mesh)
    (bind _returnvalue (`PrimitiveComponent.CreateDynamicMaterialInstance` _mesh _array_index _array_element "None"))
    (`KismetArrayLibrary.Array_Add` (`self.Materials`) _returnvalue))
  (for (_array_element_2 _array_index_2) (`MeshComponent.GetMaterials` _legs)
    (bind _returnvalue_2 (`PrimitiveComponent.CreateDynamicMaterialInstance` _legs _array_index_2 _array_element_2 "None"))
    (`KismetArrayLibrary.Array_Add` (`self.Materials`) _returnvalue_2))
  (`SceneComponent.SetVisibility` (`self.CapsuleComponent`) true true))