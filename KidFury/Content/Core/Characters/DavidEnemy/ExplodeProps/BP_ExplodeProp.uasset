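; BP_ExplodeProp is a physics prop under the DavidEnemy character, apparently debris flung out when that enemy explodes.
; On BeginPlay it applies a mass-scaled impulse to its Collision component, blending a random unit vector with a triple-weighted Direction, both scaled by Force.
; It cleans itself up through the Lifespawn lifespan or a randomized delayed destroy, whichever comes first.
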(event `self.ReceiveBeginPlay`
  (bind _collision (`self.Collision`))
  (`self.SetLifeSpan` (`self.Lifespawn`))
  (`PrimitiveComponent.AddImpulse` _collision (+ (* (`KismetMathLibrary.RandomUnitVector`) (* (`PrimitiveComponent.GetMass` _collision) (`self.Force`))) (* (* (`self.Direction`) (* (`PrimitiveComponent.GetMass` (`self.Collision`)) (`self.Force`))) 3.0)) "None" false)
  (`KismetSystemLibrary.Delay` (`KismetMathLibrary.RandomFloatInRange` 5.0 10.0))
  (`self.K2_DestroyActor`))

(fn `UserConstructionScript`)