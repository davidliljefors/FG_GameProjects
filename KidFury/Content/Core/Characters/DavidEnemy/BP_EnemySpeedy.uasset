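; BP_EnemySpeedy is the Speedy enemy variant, a child Blueprint that configures variant-specific parts on top of its parent enemy.
; Its construction script assigns the Speedy explode parts, runs the parent construction script, then passes its armour and leg guard meshes to SetArmorMaterials.
; The event graph holds only disabled placeholder events, so it adds no gameplay logic of its own.
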(fn `UserConstructionScript`
  (locals (SpeedyExplodeParts :type "/Game/Core/Characters/DavidEnemy/ExplodeProps/FExplodeProps Structure" :default (struct :`PropsToSpawn` "(None,BlueprintGeneratedClass'\"/Game/Core/Characters/DavidEnemy/ExplodeProps/BP_ExplodeProp_Speedy_2.BP_ExplodeProp_Speedy_2_C\"',BlueprintGeneratedClass'\"/Game/Core/Characters/DavidEnemy/ExplodeProps/BP_ExplodeProp_Speedy_2.BP_ExplodeProp_Speedy_2_C\"',BlueprintGeneratedClass'\"/Game/Core/Characters/DavidEnemy/ExplodeProps/BP_ExplodeProp_Speedy_2.BP_ExplodeProp_Speedy_2_C\"',BlueprintGeneratedClass'\"/Game/Core/Characters/DavidEnemy/ExplodeProps/BP_ExplodeProp_Speedy_2.BP_ExplodeProp_Speedy_2_C\"',BlueprintGeneratedClass'\"/Game/Core/Characters/DavidEnemy/ExplodeProps/BP_ExplodeProp_Speedy_3.BP_ExplodeProp_Speedy_3_C\"',BlueprintGeneratedClass'\"/Game/Core/Characters/DavidEnemy/ExplodeProps/BP_ExplodeProp_Speedy_4.BP_ExplodeProp_Speedy_4_C\"',BlueprintGeneratedClass'\"/Game/Core/Characters/DavidEnemy/ExplodeProps/BP_ExplodeProp_Speedy_4.BP_ExplodeProp_Speedy_4_C\"',BlueprintGeneratedClass'\"/Game/Core/Characters/DavidEnemy/ExplodeProps/BP_ExplodeProp_Speedy_4.BP_ExplodeProp_Speedy_4_C\"',BlueprintGeneratedClass'\"/Game/Core/Characters/DavidEnemy/ExplodeProps/BP_ExplodeProp_Speedy_4.BP_ExplodeProp_Speedy_4_C\"',BlueprintGeneratedClass'\"/Game/Core/Characters/DavidEnemy/ExplodeProps/BP_ExplodeProp_Speedy_5.BP_ExplodeProp_Speedy_5_C\"',BlueprintGeneratedClass'\"/Game/Core/Characters/DavidEnemy/ExplodeProps/BP_ExplodeProp_Speedy_5.BP_ExplodeProp_Speedy_5_C\"',BlueprintGeneratedClass'\"/Game/Core/Characters/DavidEnemy/ExplodeProps/BP_ExplodeProp_Speedy_5.BP_ExplodeProp_Speedy_5_C\"',BlueprintGeneratedClass'\"/Game/Core/Characters/DavidEnemy/ExplodeProps/BP_ExplodeProp_Speedy_5.BP_ExplodeProp_Speedy_5_C\"',BlueprintGeneratedClass'\"/Game/Core/Characters/DavidEnemy/ExplodeProps/BP_ExplodeProp_Speedy_7.BP_ExplodeProp_Speedy_7_C\"',BlueprintGeneratedClass'\"/Game/Core/Characters/DavidEnemy/ExplodeProps/BP_ExplodeProp_Speedy_7.BP_ExplodeProp_Speedy_7_C\"',BlueprintGeneratedClass'\"/Game/Core/Characters/DavidEnemy/ExplodeProps/BP_ExplodeProp_Speedy_8.BP_ExplodeProp_Speedy_8_C\"',BlueprintGeneratedClass'\"/Game/Core/Characters/DavidEnemy/ExplodeProps/BP_ExplodeProp_Speedy_8.BP_ExplodeProp_Speedy_8_C\"',BlueprintGeneratedClass'\"/Game/Core/Characters/DavidEnemy/ExplodeProps/BP_ExplodeProp_Speedy_8.BP_ExplodeProp_Speedy_8_C\"',BlueprintGeneratedClass'\"/Game/Core/Characters/DavidEnemy/ExplodeProps/BP_ExplodeProp_Speedy_8.BP_ExplodeProp_Speedy_8_C\"',BlueprintGeneratedClass'\"/Game/Core/Characters/DavidEnemy/ExplodeProps/BP_ExplodeProp_Speedy_6.BP_ExplodeProp_Speedy_6_C\"',BlueprintGeneratedClass'\"/Game/Core/Characters/DavidEnemy/ExplodeProps/BP_ExplodeProp_Speedy_6.BP_ExplodeProp_Speedy_6_C\"')")))
  (set `self.ExplodeParts` (`local.SpeedyExplodeParts`))
  (`parent.UserConstructionScript`)
  (`self.SetArmorMaterials` (`|MakeArray` (`self.SM_Armour_Speedy`) (`self.SM_LegGuards_Speedy1`) (`self.SM_LegGuards_Speedy4`) (`self.SM_LegGuards_Speedy5`) (`self.SM_LegGuards_Speedy6`))))