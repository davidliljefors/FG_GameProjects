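; Enemy bullet emitter that, once an actor overlaps it, alternates two timed attack patterns with pauses between them.
; A FlipFlop switches between a bomb volley from eight scene points and a rapid single-point stream while the root spins.
; Looping timers drive the shots, spawning BP_Projectile, while delayed open/close events gate them and restart the cycle.
; Between attacks, those timers turn the actor toward the overlapping actor in the horizontal plane.
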(event `self.ReceiveTick`
  (params (DeltaSeconds :type "Float (single-precision)"))
  (if (`self.Open`)
    (`SceneComponent.K2_AddWorldRotation` (`self.DefaultSceneRoot`) (`KismetMathLibrary.RotatorFromAxisAndAngle` (* (`SceneComponent.GetUpVector` (`self.DefaultSceneRoot`)) DeltaSeconds) 5.0) false false)))

(event `self.ReceiveBeginPlay`)

(event `Restart`
  (if (`self.Open`) :!label _label
    _
    (elif (not (`self.Open2`))
      (`/Engine/EditorBlueprintResources/StandardMacros.FlipFlop`
        (:`A`
          (`KismetSystemLibrary.K2_SetTimer` null "Fire2" 0.2 true)
          (`self.OpenBulletBomb`))
        (:`B`
          (`KismetSystemLibrary.K2_SetTimer` null "Fire" 0.05 true)
          (`self.OpenBulletHell`))))))

(event `Fire`
  (bind _returnvalue (`SceneComponent.K2_GetComponentLocation` (`self.Scene`)))
  (if (`self.Open`)
    (`|SpawnActorFromClass` "/Game/Core/Projectiles/BP_Projectile.BP_Projectile_C" (`KismetMathLibrary.MakeTransform` _returnvalue (`KismetMathLibrary.Conv_VectorToRotator` (`SceneComponent.GetForwardVector` (`self.Scene`)))) "Undefined" "OverrideRootScale" null 600.0 null)
    (elif (not (`self.Open2`))
      (bind (_returnvalue_x _returnvalue_y) (`KismetMathLibrary.BreakVector` (`self.K2_GetActorLocation` (stale `self.ReceiveActorBeginOverlap` OtherActor))))
      (`self.K2_SetActorRotation` (`KismetMathLibrary.FindLookAtRotation` (`KismetMathLibrary.MakeVector` (.x _returnvalue) (.y _returnvalue)) (`KismetMathLibrary.MakeVector` _returnvalue_x _returnvalue_y)) :!label _label_2))))

(event `self.ReceiveActorBeginOverlap`
  (params (OtherActor :type "Actor Object Reference"))
  (goto _label))

(event `Fire2`
  (if (`self.Open2`)
    (`|ExecutionSequence`
      (:`then_0`
        (`self.NewMacro_0` (`self.Scene1`)))
      (:`then_1`
        (`self.NewMacro_0` (`self.Scene2`)))
      (:`then_2`
        (`self.NewMacro_0` (`self.Scene3`)))
      (:`then_3`
        (`self.NewMacro_0` (`self.Scene4`)))
      (:`then_4`
        (`self.NewMacro_0` (`self.Scene5`)))
      (:`then_5`
        (`self.NewMacro_0` (`self.Scene6`)))
      (:`then_6`
        (`self.NewMacro_0` (`self.Scene7`)))
      (:`then_7`
        (`self.NewMacro_0` (`self.Scene`))))
    (elif (`self.Open2`)
      _
      (elif (not (`self.Open`))
        (goto _label_2)))))

(event `OpenBulletHell`
  ;[1 1 1] Comment
  (set `self.Open` true)
  (`KismetSystemLibrary.Delay` 3.0)
  (`self.CloseBulletHell`))

(event `CloseBulletHell`
  ;[1 1 1] Comment
  (set `self.Open` false)
  (`KismetSystemLibrary.Delay` 3.0)
  (`self.Restart`))

(event `OpenBulletBomb`
  ;[1 1 1] Comment
  (set `self.Open2` true)
  (`KismetSystemLibrary.Delay` 3.0)
  (`self.CloseBulletBomb`))

(event `CloseBulletBomb`
  ;[1 1 1] Comment
  (set `self.Open2` false)
  (`KismetSystemLibrary.Delay` 3.0)
  (`self.Restart`))

(fn `NewFunction_0`
  (params (Target :type "SceneComponent Object Reference") (NewParam :type "Vector Structure")))

(fn `RotateActorAroundPoint`
  (params (RotateScne :type "Actor Object Reference") (targetRotate :type "Actor Object Reference") (Radius :type "Vector Structure") (Location :type "Vector Structure") (angle :type "Float (double-precision)") (RotationRate :type "Float (double-precision)")))

(fn `UserConstructionScript`)