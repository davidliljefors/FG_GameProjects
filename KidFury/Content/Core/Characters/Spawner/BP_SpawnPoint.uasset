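; Spawn point that creates AI pawns at random navmesh locations within a radius of its Arrow, facing the arrow's direction.
; Spawn uses a valid override group for per-entry classes and counts, otherwise its own default class and count.
; Override spawns pick navigable points while default spawns pick reachable ones; both add to and return SpawnedPawns.
; The Spawn event in the event graph is an empty stub.
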(event `Spawn_1_1`
  (params (SpawnData :type "/Game/Core/Characters/Spawner/FSpawnData Structure")))

(fn `Spawn`
  (params (OverrideSpawnData :type "/Game/Core/Characters/Spawner/FSpawnGroup Structure"))
  (returns (ReturnValue :type "Array of Pawn Object Reference"))
  (locals (SpawnedPawns :type "Array of Pawn Object Reference"))
  (bind _arrow (`self.Arrow`))
  (bind _arrow_2 (`self.Arrow`))
  (if (`/Game/Core/World/BPF_Utilities.IsValidSpawnGroup` OverrideSpawnData)
    (for _array_element (`.SpawnGroup_3_F910D11D478B03F3E2BFEBA4C846180F` (break `/Game/Core/Characters/Spawner/FSpawnGroup` OverrideSpawnData))
      (if (`/Game/Core/World/BPF_Utilities.IsValidSpawnData` _array_element)
        (bind (_class _numtospawn) (break `/Game/Core/Characters/Spawner/FSpawnData` _array_element))
        (for _ (range _numtospawn)
          (bind _returnvalue (`AIBlueprintHelperLibrary.SpawnAIFromClass` _class null (`NavigationSystemV1.K2_GetRandomLocationInNavigableRadius` (`SceneComponent.K2_GetComponentLocation` _arrow_2) (`self.SpawnRadius`) null null) (`SceneComponent.K2_GetComponentRotation` _arrow_2) true))
          (`KismetArrayLibrary.Array_AddUnique` (`local.SpawnedPawns`) _returnvalue))))
    (return (`local.SpawnedPawns`))
    (else
      (for _ (range (`self.NumToSpawn`))
        (bind _returnvalue_2 (`AIBlueprintHelperLibrary.SpawnAIFromClass` (`self.Spawn Class`) null (`NavigationSystemV1.K2_GetRandomReachablePointInRadius` (`SceneComponent.K2_GetComponentLocation` _arrow) (`self.SpawnRadius`) null null) (`SceneComponent.K2_GetComponentRotation` _arrow) true))
        (`KismetArrayLibrary.Array_AddUnique` (`local.SpawnedPawns`) _returnvalue_2))
      (return (`local.SpawnedPawns`)))))

(fn `UserConstructionScript`)