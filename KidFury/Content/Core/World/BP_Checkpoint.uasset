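; Checkpoint actor that saves player progress to a BP_SaveData slot when its trigger is overlapped, then destroys itself.
; With ShouldLoad on, it records player location, coins, last spawner, gamepad and audio settings.
; It also reads BP_LightBlend lighting, but writes it to a separately loaded "Check" save object that is never saved afterward.
; With ShouldLoad off, it clears the Load flag and saves to an empty slot name.
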(event `self.Trigger.OnComponentBeginOverlap`
  (params (OverlappedComponent :type "PrimitiveComponent Object Reference") (OtherActor :type "Actor Object Reference") (OtherComp :type "PrimitiveComponent Object Reference") (OtherBodyIndex :type Integer) (bFromSweep :type Boolean) (SweepResult :type "HitResult Structure (by ref)"))
  (if (`self.bShouldLoad`)
    (`|ExecutionSequence`
      (:`then_0`
        (bind _asgp2character (cast `GP2Character` (`GameplayStatics.GetPlayerCharacter` 0)))
        (set `self.PlayerLocation` (`self.K2_GetActorLocation` _asgp2character))
        (bind _asbp_player_character (cast `/Game/Core/Characters/Player/BP_PlayerCharacter` (`GameplayStatics.GetPlayerCharacter` 0)))
        (set `self.bGamepadEnabled` (`GP2Character.bUseGamepad` _asbp_player_character))
        (bind (_currentdirecttemperature _currentdirectcolor _currentdirectintensity _currentskycolor _currentskyintensity _blendiscomplete) (`self.GetLightblendVariables`))
        (`self.SetLightblendVariables` _currentdirecttemperature _currentdirectcolor _currentdirectintensity _currentskycolor _currentskyintensity _blendiscomplete)
        (bind _ashud_gp2 (cast `/Game/UI/HUD_GP2` (`PlayerController.GetHUD` (`GameplayStatics.GetPlayerController` 0))))
        (set `self.bIsSFXEnabled` (`/Game/UI/HUD_GP2.IsSFX_Enabled` _ashud_gp2))
        (set `self.bIsMusicEnabled` (`/Game/UI/HUD_GP2.IsMusicEnabled` _ashud_gp2))
        (bind _returnvalue (`GameplayStatics.DoesSaveGameExist` (`self.SaveName`)))
        (if _returnvalue
          (bind _returnvalue_2 (`GameplayStatics.LoadGameFromSlot` (`self.SaveName`)))
          (bind _asbp_save_data (cast `/Game/Core/World/BP_SaveData` _returnvalue_2))
          (`BlueprintMapLibrary.Map_Add` (`/Game/Core/World/BP_SaveData.Encountermap` _asbp_save_data) (`self.LastSpawner`) true)
          (else
            (bind _returnvalue_3 (`GameplayStatics.CreateSaveGameObject` "/Game/Core/World/BP_SaveData.BP_SaveData_C"))))
        (`GameplayStatics.SaveGameToSlot` _returnvalue_3 (`self.SaveName`)))
      (:`then_1`
        (bind _returnvalue_4 (`GameplayStatics.DoesSaveGameExist` (`self.SaveName`)))
        (if _returnvalue_4
          (bind _returnvalue_5 (`GameplayStatics.LoadGameFromSlot` (`self.SaveName`)))
          (bind _asbp_save_data_2 (cast `/Game/Core/World/BP_SaveData` _returnvalue_5))
          (set `/Game/Core/World/BP_SaveData.Coins` (`self.Coins`) _asbp_save_data_2)
          (set `/Game/Core/World/BP_SaveData.PlayerLocation` (`self.PlayerLocation`) _asbp_save_data_2)
          (set `/Game/Core/World/BP_SaveData.bLoad` true _asbp_save_data_2)
          (`BlueprintMapLibrary.Map_Add` (`/Game/Core/World/BP_SaveData.Encountermap` _asbp_save_data_2) (`self.LastSpawner`) true)
          (set `/Game/Core/World/BP_SaveData.bGamepadEnabled` (`self.bGamepadEnabled`) _asbp_save_data_2)
          (`self.SetSaveLightblendVariables` (`self.LightColor`) (`self.Intensity`) (`self.Temprature`) (`self.SkyColor`) (`self.SkyIntensity`) (`self.bBlendIsComplete`))
          (set `/Game/Core/World/BP_SaveData.bIsSFXEnabled` (`self.bIsSFXEnabled`) _asbp_save_data_2)
          (set `/Game/Core/World/BP_SaveData.bIsMusicEnabled` (`self.bIsMusicEnabled`) _asbp_save_data_2)
          (`GameplayStatics.SaveGameToSlot` _asbp_save_data_2 (`self.SaveName`))
          (else
            (bind _returnvalue_6 (`GameplayStatics.CreateSaveGameObject` "/Game/Core/World/BP_SaveData.BP_SaveData_C"))
            (set `/Game/Core/World/BP_SaveData.PlayerLocation` (`self.PlayerLocation`) _returnvalue_6)
            (set `/Game/Core/World/BP_SaveData.Coins` (`self.Coins`) _returnvalue_6)
            (set `/Game/Core/World/BP_SaveData.bLoad` true _returnvalue_6)
            (`BlueprintMapLibrary.Map_Add` (`/Game/Core/World/BP_SaveData.Encountermap` _returnvalue_6) (`self.LastSpawner`) true)
            (set `/Game/Core/World/BP_SaveData.bGamepadEnabled` (`self.bGamepadEnabled`) _returnvalue_6)
            (set `/Game/Core/World/BP_SaveData.bIsSFXEnabled` (`self.bIsSFXEnabled`) _returnvalue_6)
            (set `/Game/Core/World/BP_SaveData.bIsMusicEnabled` (`self.bIsMusicEnabled`) _returnvalue_6)
            (`self.SetSaveLightblendVariables` (`self.LightColor`) (`self.Intensity`) (`self.Temprature`) (`self.SkyColor`) (`self.SkyIntensity`) (`self.bBlendIsComplete`))
            (`GameplayStatics.SaveGameToSlot` _returnvalue_6 (`self.SaveName`))))
        (`KismetSystemLibrary.Delay` 0.2)
        (`self.K2_DestroyActor`)))
    (else
      (bind _returnvalue_7 (`GameplayStatics.LoadGameFromSlot` (`self.SaveName`)))
      (bind _asbp_save_data_3 (cast `/Game/Core/World/BP_SaveData` _returnvalue_7))
      (set `/Game/Core/World/BP_SaveData.bLoad` false _asbp_save_data_3)
      (`GameplayStatics.SaveGameToSlot` _asbp_save_data_3))))

(fn `GetLightblendVariables`
  (returns (CurrentDirectTemperature :type "Float (double-precision)") (CurrentDirectColor :type "LinearColor Structure") (CurrentDirectIntensity :type "Float (double-precision)") (CurrentSkyColor :type "LinearColor Structure") (CurrentSkyIntensity :type "Float (double-precision)") (BlendIsComplete :type Boolean))
  (bind _returnvalue (`GameplayStatics.GetActorOfClass` "/Game/Core/World/BP_LightBlend.BP_LightBlend_C"))
  (return (`/Game/Core/World/BP_LightBlend.CurrentDirectTemperature` _returnvalue) (`/Game/Core/World/BP_LightBlend.CurrentDirectColor` _returnvalue) (`/Game/Core/World/BP_LightBlend.CurrentDirectIntensity` _returnvalue) (`/Game/Core/World/BP_LightBlend.CurrentSkyColor` _returnvalue) (`/Game/Core/World/BP_LightBlend.CurrentSkyIntensity` _returnvalue) (`/Game/Core/World/BP_LightBlend.BlendIsComplete` _returnvalue)))

(fn `SetLightblendVariables`
  (params (Temprature :type "Float (double-precision)") (LightColor :type "LinearColor Structure") (Intensity :type "Float (double-precision)") (SkyColor :type "LinearColor Structure") (SkyIntensity :type "Float (double-precision)") (bBlendIsComplete :type Boolean))
  (set `self.LightColor` LightColor)
  (set `self.Intensity` Intensity)
  (set `self.Temprature` Temprature)
  (set `self.SkyColor` SkyColor)
  (set `self.SkyIntensity` SkyIntensity)
  (set `self.bBlendIsComplete` bBlendIsComplete)
  (return))

(fn `SetSaveLightblendVariables`
  (params (LightColor :type "LinearColor Structure") (Intensity :type "Float (double-precision)") (Temprature :type "Float (double-precision)") (SkyColor :type "LinearColor Structure") (SkyIntensity :type "Float (double-precision)") (bBlendIsComplete :type Boolean))
  (bind _returnvalue (`GameplayStatics.DoesSaveGameExist` "Check"))
  (if _returnvalue
    (bind _returnvalue_2 (`GameplayStatics.LoadGameFromSlot` "Check"))
    (else
      (bind _returnvalue_3 (`GameplayStatics.CreateSaveGameObject` "/Game/Core/World/BP_SaveData.BP_SaveData_C"))
      (`GameplayStatics.SaveGameToSlot` _returnvalue_3 "Check")))
  (bind _asbp_save_data (cast `/Game/Core/World/BP_SaveData` _returnvalue_2))
  (set `/Game/Core/World/BP_SaveData.LightColor` LightColor _asbp_save_data)
  (set `/Game/Core/World/BP_SaveData.Intensity` Intensity _asbp_save_data)
  (set `/Game/Core/World/BP_SaveData.Temprature` Temprature _asbp_save_data)
  (set `/Game/Core/World/BP_SaveData.SkyColor` SkyColor _asbp_save_data)
  (set `/Game/Core/World/BP_SaveData.SkyIntensity` SkyIntensity _asbp_save_data)
  (set `/Game/Core/World/BP_SaveData.bBlendIsComplete` bBlendIsComplete _asbp_save_data))

(fn `UserConstructionScript`)