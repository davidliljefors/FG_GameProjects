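; BP_LightBlend shifts the level's directional light and skylight toward new values as the player nears a BP_LightBlendTarget.
; BeginPlay caches default lighting; blending starts then or on the player's first trigger overlap, per ShouldActivateByTrigger.
; Tick normalizes distance to the target into a forward-only alpha, lerping color, intensity, temperature and sun rotation until near completion.
; Save-data restore and timer-based BlendLight paths are disconnected.
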(event `SetCurrentValues`
  (bind _lightcomponent (`SkyLight.LightComponent` (`self.LevelSkyLight`)))
  (bind _lightcomponent_2 (`Light.LightComponent` (`self.DirectionalLight`)))
  (set `self.CurrentSkyColor` (`LightComponentBase.GetLightColor` _lightcomponent))
  (set `self.CurrentSkyIntensity` (`LightComponentBase.Intensity` _lightcomponent))
  (set `self.CurrentDirectColor` (`LightComponentBase.GetLightColor` _lightcomponent_2))
  (set `self.CurrentDirectTemperature` (`LightComponentBase.Intensity` _lightcomponent_2))
  (set `self.CurrentDirectIntensity` (`LightComponent.Temperature` _lightcomponent_2)))

(event `self.TriggerVolume.OnComponentBeginOverlap`
  (params (OverlappedComponent :type "PrimitiveComponent Object Reference") (OtherActor :type "Actor Object Reference") (OtherComp :type "PrimitiveComponent Object Reference") (OtherBodyIndex :type Integer) (bFromSweep :type Boolean) (SweepResult :type "HitResult Structure (by ref)"))
  ;[1 1 1 1 69] Skiten som springer
  ;;[1 1 1] If player should activate by trigger
  (if (and (== OtherActor (`GameplayStatics.GetPlayerPawn` 0)) (`self.ShouldActivateByTrigger`))
    (`/Engine/EditorBlueprintResources/StandardMacros.DoOnce` false
      (:`Completed`
        (bind _returnvalue (`GameplayStatics.GetActorOfClass` "/Game/Core/World/BP_LightBlendTarget.BP_LightBlendTarget_C"))
        (set `self.LightBlendTarget` _returnvalue)
        (set `self.DistanceToFinalBlend` (`self.GetDistanceToFinalBlend`))
        (`self.SetActorTickEnabled` true)
        (set `self.HasActivatedTrigger` true)))))

(event `self.ReceiveBeginPlay`
  ;[1 1 1 1 69] Skiten som springer
  ;;[1 1 1] Get skylight and Directional light from scene
  (`self.GetAllActors`)
  (`self.SetActorTickEnabled` false)
  (set `self.PlayerTest` (`GameplayStatics.GetPlayerCharacter` 0))
  (`self.GetDefaultLightValues`)
  (if (not (`self.ShouldActivateByTrigger`))
    (bind _returnvalue (`GameplayStatics.GetActorOfClass` "/Game/Core/World/BP_LightBlendTarget.BP_LightBlendTarget_C"))
    (set `self.LightBlendTarget` _returnvalue)
    (set `self.DistanceToFinalBlend` (`self.GetDistanceToFinalBlend`))
    (`self.SetActorTickEnabled` true)))

(event `SetLights`
  (bind _lightcomponent (`Light.LightComponent` (`self.DirectionalLight`)))
  (bind _lightcomponent_2 (`SkyLight.LightComponent` (`self.LevelSkyLight`)))
  (`|ExecutionSequence`
    (:`then_0`
      (`LightComponent.SetIntensity` _lightcomponent (`self.DefaultDirectIntens`))
      (`LightComponent.SetLightColor` _lightcomponent (`KismetMathLibrary.Conv_ColorToLinearColor` (`self.DefaultDirectLight`)) true)
      (`LightComponent.SetTemperature` _lightcomponent (`self.DefaultDirectTemp`)))
    (:`then_1`
      (`SkyLightComponent.SetIntensity` _lightcomponent_2 (`self.DefaultSkyIntens`))
      (`SkyLightComponent.SetLightColor` _lightcomponent_2 (`self.DefaultSkyColor`)))))

(event `GetDefaultLightValues`
  (bind _lightcomponent (`Light.LightComponent` (`self.DirectionalLight`)))
  (bind _lightcomponent_2 (`SkyLight.LightComponent` (`self.LevelSkyLight`)))
  ;[1 1 1 1 69] Skiten som springer
  ;;[1 1 1] Get the default values of each light in scene
  (`|ExecutionSequence`
    (:`then_0`
      (set `self.DefaultDirectTemp` (`LightComponent.Temperature` _lightcomponent))
      (set `self.DefaultDirectIntens` (`LightComponentBase.Intensity` _lightcomponent))
      (set `self.DefaultDirectRot` (`SceneComponent.K2_GetComponentRotation` _lightcomponent))
      (set `self.DefaultDirectLight` (`LightComponentBase.LightColor` _lightcomponent)))
    (:`then_1`
      (set `self.DefaultSkyIntens` (`LightComponentBase.Intensity` _lightcomponent_2))
      (set `self.DefaultSkyColor` (`LightComponentBase.GetLightColor` _lightcomponent_2)))))

(event `BlendLight`
  (bind _directionallight (`self.DirectionalLight`))
  (bind _lightcomponent (`Light.LightComponent` _directionallight))
  (bind _lightcomponent_2 (`SkyLight.LightComponent` (`self.LevelSkyLight`)))
  ;[1 1 1] Comment
  (set `self.DeltaTimetick` (`GameplayStatics.GetWorldDeltaSeconds`))
  (`|ExecutionSequence`
    (:`then_0`
      (`SkyLightComponent.SetIntensity` _lightcomponent_2 (`KismetMathLibrary.FInterpTo` (`LightComponentBase.Intensity` _lightcomponent_2) (`self.InNewSkyIntensity`) (`self.DeltaTimetick`) (`self.TimeToBlend`))))
    (:`then_1`
      (`LightComponent.SetTemperature` _lightcomponent (`KismetMathLibrary.FInterpTo` (`LightComponent.Temperature` _lightcomponent) (`self.InNewDirectionalTemperature`) (`self.DeltaTimetick`) (`self.TimeToBlend`)))
      (`LightComponent.SetIntensity` _lightcomponent (`KismetMathLibrary.FInterpTo` (`LightComponentBase.Intensity` _lightcomponent) (`self.InNewDirectionalIntensity`) (`self.DeltaTimetick`) (`self.TimeToBlend`)))
      (`self.K2_SetActorRotation` _directionallight (`KismetMathLibrary.RInterpTo_Constant` (`self.rotation`) (`self.InNewDirectionalRot`) (`self.DeltaTimetick`) (`self.TimeToBlend`)) false))))

(event `self.ReceiveTick`
  (params (DeltaSeconds :type "Float (single-precision)"))
  (bind _returnvalue (- 1.0 (`KismetMathLibrary.NormalizeToRange` (`self.GetDistanceToFinalBlend`) (`self.DistanceToFinalBlend`) 100.0)))
  ;[1 1 1 1 69] Skiten som springer
  ;;[1 1 1] Normalized range n shit
  (if (`self.BlendIsComplete`)
    (`self.SetActorTickEnabled` false)
    (elif (not (< _returnvalue (`self.NormalizedDistance`)))
      (bind _output_get (set `self.NormalizedDistance` _returnvalue))
      (if (>= _output_get 0.93)
        (set `self.BlendIsComplete` true)
        (else
          (`self.LerpLightValues`))))))

(event `LerpLightValues`
  (bind _directionallight (`self.DirectionalLight`))
  (bind _normalizeddistance (`self.NormalizedDistance`))
  (bind _lightcomponent (`SkyLight.LightComponent` (`self.LevelSkyLight`)))
  (bind _lightcomponent_2 (`Light.LightComponent` _directionallight))
  ;[1 1 1 1 69] Skiten som springer
  ;;[1 1 1] Lots a lerps
  (`|ExecutionSequence`
    (:`then_0`
      (bind _output_get (set `self.CurrentSkyIntensity` (`KismetMathLibrary.Lerp` (`self.DefaultSkyIntens`) (`self.InNewSkyIntensity`) _normalizeddistance)))
      (`SkyLightComponent.SetIntensity` _lightcomponent _output_get)
      (bind _output_get_2 (set `self.CurrentSkyColor` (`KismetMathLibrary.LinearColorLerp` (`self.DefaultSkyColor`) (`self.InNewSkyColor`) _normalizeddistance)))
      (`SkyLightComponent.SetLightColor` _lightcomponent _output_get_2))
    (:`then_1`
      (bind _output_get_3 (set `self.CurrentDirectTemperature` (`KismetMathLibrary.Lerp` (`self.DefaultDirectTemp`) (`self.InNewDirectionalTemperature`) (`self.NormalizedDistance`))))
      (`LightComponent.SetTemperature` _lightcomponent_2 _output_get_3)
      (bind _output_get_4 (set `self.CurrentDirectIntensity` (`KismetMathLibrary.Lerp` (`self.DefaultDirectIntens`) (`self.InNewDirectionalIntensity`) (`self.NormalizedDistance`))))
      (`LightComponent.SetIntensity` _lightcomponent_2 _output_get_4)
      (`self.K2_SetActorRotation` _directionallight (`KismetMathLibrary.RLerp` (`self.DefaultDirectRot`) (`self.InNewDirectionalRot`) (`self.NormalizedDistance`)) false)
      (bind _output_get_5 (set `self.CurrentDirectColor` (`KismetMathLibrary.LinearColorLerp` (`KismetMathLibrary.Conv_ColorToLinearColor` (`self.DefaultDirectLight`)) (`self.InNewDirectColor`) (`self.NormalizedDistance`))))
      (`LightComponent.SetLightColor` _lightcomponent_2 _output_get_5 true))))

(fn `GetAllActors`
  (bind _outactors (`GameplayStatics.GetAllActorsOfClass` "/Script/Engine.DirectionalLight"))
  (set `self.DirectionalLight` (`|GetArrayItem` _outactors))
  (bind _outactors_2 (`GameplayStatics.GetAllActorsOfClass` "/Script/Engine.SkyLight"))
  (set `self.LevelSkyLight` (`|GetArrayItem` _outactors_2))
  (bind _outactors_3 (`GameplayStatics.GetAllActorsOfClass` "/Game/Core/Characters/Player/BP_PlayerCharacter.BP_PlayerCharacter_C"))
  (set `self.Player` (`|GetArrayItem` _outactors_3)))

(fn `GetDistanceToFinalBlend`
  (returns (ReturnValue :type "Float (double-precision)"))
  (return (`KismetMathLibrary.Vector_Distance` (`SceneComponent.K2_GetComponentLocation` (`Character.CapsuleComponent` (`self.PlayerTest`))) (`SceneComponent.K2_GetComponentLocation` (`/Game/Core/World/BP_LightBlendTarget.DefaultSceneRoot` (`self.LightBlendTarget`))))))

(fn `GetLightBlendTarget`)

(fn `UserConstructionScript`)