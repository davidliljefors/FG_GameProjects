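; BP_AmbienceSound is an actor that fades in an ambience Audio component when the main or pause menu is showing.
; BeginPlay caches the player's HUD_GP2, and Tick polls whether either menu widget is in the viewport.
; A DoOnce with no reset limits the fade-in to the first detection.
; A fade-out node exists but is unconnected, so it never runs.
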(event `self.ReceiveBeginPlay`
  (bind _ashud_gp2 (cast `/Game/UI/HUD_GP2` (`PlayerController.GetHUD` (`GameplayStatics.GetPlayerController` 0))))
  (set `self.HUD` _ashud_gp2))

(event `self.ReceiveTick`
  (params (DeltaSeconds :type "Float (single-precision)"))
  (bind _hud (`self.HUD`))
  (if (or (`Widget.IsInViewport` (`/Game/UI/HUD_GP2.MainMenu` _hud)) (`Widget.IsInViewport` (`/Game/UI/HUD_GP2.PauseMenu` _hud)))
    (`/Engine/EditorBlueprintResources/StandardMacros.DoOnce` false
      (:`Completed`
        (`AudioComponent.FadeIn` (`self.Audio`) 1.0 1.0 0.0 "Linear")))))

(fn `UserConstructionScript`)