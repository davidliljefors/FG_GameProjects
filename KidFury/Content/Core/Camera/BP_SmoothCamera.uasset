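; Smoothed player-follow camera that leans toward the aim direction and offers a combat zoom, registering itself on BP_PlayerCharacter at BeginPlay.
; Each tick offsets the view target by gamepad right stick or mouse distance from screen center, then lerps the spring arm toward it with capped delta time.
; ZoomOut and ZoomIn play and reverse a timeline that blends arm length toward the combat distance, with alpha scaled by frame delta.
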(event `self.ReceiveBeginPlay`
  (bind _asbp_player_character (cast `/Game/Core/Characters/Player/BP_PlayerCharacter` (`GameplayStatics.GetPlayerCharacter` 0)))
  (set `/Game/Core/Characters/Player/BP_PlayerCharacter.SmoothCamera` self _asbp_player_character)
  (bind _asbp_player_character_2 (cast `/Game/Core/Characters/Player/BP_PlayerCharacter` (`GameplayStatics.GetPlayerCharacter` 0)))
  (set `self.Player` _asbp_player_character_2)
  (set `self.TargetCombatZoom` (+ (`SpringArmComponent.TargetArmLength` (`self.SpringArm`)) (`self.CombatZoomDistance`))))

(event `self.ReceiveTick`
  (params (DeltaSeconds :type "Float (single-precision)"))
  (bind _offset (`self.Offset`))
  (bind _player (`self.Player`))
  (bind _returnvalue (`self.K2_GetActorLocation` _player))
  (if (`GP2Character.bUseGamepad` _player)
    (`self.SetViewTarget` _returnvalue _offset (`self.GetOffsetFromVec2D` (`/Game/Core/Characters/Player/BP_PlayerCharacter.GamepadRightStick` _player)) 125.0)
    (else
      (`self.SetViewTarget` _returnvalue _offset (`self.GetMouseOffsetNormalized`) 125.0)))
  (`SceneComponent.K2_SetWorldLocation` (`self.SpringArm`) (`KismetMathLibrary.VLerp` (`SceneComponent.K2_GetComponentLocation` (`self.SpringArm`)) (`self.TargetView`) (* (`KismetMathLibrary.FMin` DeltaSeconds 0.1) (`self.LerpSpeed`))) false false)
  (set `SpringArmComponent.TargetArmLength` (`self.TargetSpringArmLength`) (`self.SpringArm`)))

(event `ZoomOut`
  (set `self.CurrentSpringArmLength` (`SpringArmComponent.TargetArmLength` (`self.SpringArm`)))
  (bind (_direction _alpha) (`Timeline|Zoom` :!via `PlayFromStart` :!label _label)
    (:`Update`
      (set `self.TargetSpringArmLength` (`KismetMathLibrary.Lerp` (`self.CurrentSpringArmLength`) (`self.TargetCombatZoom`) (* _alpha (`GameplayStatics.GetWorldDeltaSeconds`)))))))

(event `ZoomIn`
  (goto _label :!via `Reverse`))

(fn `GetMouseOffsetNormalized`
  (returns (Offset :type "Vector Structure"))
  (bind _returnvalue (`WidgetLayoutLibrary.GetViewportSize`))
  (bind (_x _y) (`KismetMathLibrary.BreakVector2D` _returnvalue))
  (bind _returnvalue_2 (`WidgetLayoutLibrary.GetMousePositionOnViewport`))
  (bind (_returnvalue_x _returnvalue_y) (`KismetMathLibrary.BreakVector2D` (- _returnvalue_2 (/ _returnvalue 2.0))))
  (return (`KismetMathLibrary.Vector_ClampSizeMax` (`KismetMathLibrary.MakeVector` (* (/ (* _returnvalue_y -1.0) _y) 2.0) (* (/ _returnvalue_x _x) 2.0)) 1.0)))

(fn `GetOffsetFromVec2D`
  (params (Input :type "Vector2D Structure"))
  (returns (Offset :type "Vector Structure"))
  (return (`KismetMathLibrary.Vector_ClampSizeMax` (`KismetMathLibrary.MakeVector` (* Input_Y -1.0) Input_X) 1.0)))

(fn `SetViewTarget`
  (params (ActorLoc :type "Vector Structure") (CameraLoc :type "Vector Structure") (LookDir :type "Vector Structure") (Length :type "Float (double-precision)" :default 100.0))
  (set `self.TargetView` (+ ActorLoc CameraLoc (* LookDir Length)))
  (return))

(fn `UserConstructionScript`)