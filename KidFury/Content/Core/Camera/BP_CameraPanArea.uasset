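; BP_CameraPanArea is a trigger area that plays a one-time camera pan when the player character enters it.
; It caches the player and BP_SmoothCamera's starting rotation on BeginPlay.
; On overlap it disables player input and a timeline lerps the camera's world rotation to CameraTargetRot.
; When that finishes, the timeline reverses to pan back, then restores input, with DoOnce and IsPanned preventing repeats.
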(event `self.ReceiveBeginPlay`
  (bind _returnvalue (`GameplayStatics.GetActorOfClass` "/Game/Core/Characters/Player/BP_PlayerCharacter.BP_PlayerCharacter_C"))
  (set `self.Player` _returnvalue)
  (bind _returnvalue_2 (`GameplayStatics.GetActorOfClass` "/Game/Core/Camera/BP_SmoothCamera.BP_SmoothCamera_C"))
  (if (`KismetSystemLibrary.IsValid` _returnvalue_2)
    (bind _output_get (set `self.SmoothCamera` _returnvalue_2))
    (set `self.CameraDefaultRot` (`SceneComponent.K2_GetComponentRotation` (`/Game/Core/Camera/BP_SmoothCamera.SmoothCamera` _output_get)))))

(event `self.TriggerVolume.OnComponentBeginOverlap`
  (params (OverlappedComponent :type "PrimitiveComponent Object Reference") (OtherActor :type "Actor Object Reference") (OtherComp :type "PrimitiveComponent Object Reference") (OtherBodyIndex :type Integer) (bFromSweep :type Boolean) (SweepResult :type "HitResult Structure (by ref)"))
  (if (and (== OtherActor (`GameplayStatics.GetPlayerCharacter` 0)) (not (`self.IsPanned`)))
    (`/Engine/EditorBlueprintResources/StandardMacros.DoOnce` false
      (:`Completed`
        (set `GP2Character.bUseInput` false (`self.Player`))
        (bind (_direction _cameralerp) (`Timeline|LerpCameraRot` :!via `PlayFromStart` :!label _label)
          (:`Update`
            (`SceneComponent.K2_SetWorldRotation` (`/Game/Core/Camera/BP_SmoothCamera.SmoothCamera` (`self.SmoothCamera`)) (`KismetMathLibrary.RLerp` (`self.CameraDefaultRot`) (`self.CameraTargetRot`) _cameralerp) false false))
          (:`Finished`
            (if (`self.IsPanned`)
              (set `GP2Character.bUseInput` true (`self.Player`))
              (else
                (`self.PanBack`)
                (set `self.IsPanned` true)))))))))

(event `PanBack`
  (goto _label :!via `ReverseFromEnd`))

(fn `UserConstructionScript`)